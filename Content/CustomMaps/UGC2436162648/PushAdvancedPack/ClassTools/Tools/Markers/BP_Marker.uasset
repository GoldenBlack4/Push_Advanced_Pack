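; BP_Marker is a temporary team marker for Pavlov: a textured plane shown to local players on the matching team, with a one-time 2D sound for them.
; After a short delay the authority optionally flips TeamID, and all instances set lifespan and material.
; A looping timer updates visibility by team, defaulting to visible if player status lookup fails.
; Tick yaws the marker relative to the local pawn and scales and raises it with distance.
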(event Custom|Check
  (bind (_playerstatus _bsucceeded) (Class|PavlovProxyStatics|GetPavlovPlayerStatusbyPawn (Game|Player|GetPlayerPawn 0)))
  (if _bsucceeded
    (Rendering|SetActorHiddenInGame (not (== (Variables|Default|GetTeamID) (.TeamId (Utilities|Struct|BreakPavlovPlayerStatus _playerstatus)))))
    (else
      (Rendering|SetActorHiddenInGame false)))
  (Utilities|FlowControl|DoOnce false
    (:Completed
      (if (== (Variables|Default|GetTeamID) (.TeamId (Utilities|Struct|BreakPavlovPlayerStatus _playerstatus)))
        (Audio|PlaySound2D (Variables|Default|GetSound) 0.25 1.0 0.0 0 (Game|Player|GetPlayerPawn 0))))))

(event EventTick
  (params (DeltaSeconds :type Float%20%28single-precision%29))
  (bind _returnvalue (Game|Player|GetPlayerPawn 0))
  (bind _plane (Variables|Default|GetPlane))
  (bind _returnvalue_2 (Transformation|GetWorldLocation _plane))
  (bind _returnvalue_3 (Transformation|GetDistanceTo _returnvalue))
  (bind _returnvalue_4 (/ _returnvalue_3 1.5e+03))
  (bind _returnvalue_5 (Math|Float|Clamp(Float) _returnvalue_4 0.5 5.0))
  (Transformation|SetActorRotation (Math|Rotator|MakeRotator 0.0 0.0 (+ (.Yaw (Math|Rotator|BreakRotator (Math|Rotator|FindLookatRotation (Transformation|GetActorLocation (Game|Player|GetPlayerPawn 0)) (Transformation|GetWorldLocation (Variables|Default|GetPlane))))) 9e+01)))
  (Transformation|SetWorldScale3D _plane (Math|Vector|MakeVector _returnvalue_5 _returnvalue_5 _returnvalue_5))
  (Transformation|SetWorldLocation _plane (Math|Vector|MakeVector (.x _returnvalue_2) (.y _returnvalue_2) (+ (Math|Float|Clamp(Float) _returnvalue_3 2e+02 1e+03) (.z (Transformation|GetActorLocation)))) false false))

(event EventBeginPlay
  (Utilities|FlowControl|Delay 0.1)
  (Utilities|FlowControl|Sequence
    (:then_0
      (Networking|SwitchHasAuthority
        (:Authority
          (CallFunction|SwitchonTDM))))
    (:then_1
      (Actor|SetLifeSpan (Variables|Default|GetLifeSpan))
      (Rendering|Material|SetMaterial (Variables|Default|GetPlane) 0 (Variables|Default|GetMaterial))
      (Utilities|Time|SetTimerbyEvent (delegate Custom|Check) 0.1 true))))

(fn ConstructionScript)

(fn SwitchonTDM
  (if (Variables|Default|GetTeamIDSwitched)
    (if (== (Variables|Default|GetTeamID) 0)
      (Variables|Default|SetTeamID 1)
      (else
        (Variables|Default|SetTeamID 0)))))