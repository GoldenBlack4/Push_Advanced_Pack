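; BP_Backpack is a parachute backpack actor for a pawn, with a German or US look chosen by team.
; On BeginPlay the authority takes PawnOwner as owner and, after a short delay, spawns a zero-scale BP_Parachute at the backpack's AttachPoint socket.
; It passes the parachute its pawn, opening sound and backpack reference, attaches it to the pawn, then calls MulticastMesh to set the team's mesh and material.
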(event Custom|MulticastMesh
  (params (TeamID :type Integer))
  (Components|StaticMesh|SetStaticMesh (Variables|Default|GetBackpack) (Utilities|Select :Index TeamID :Option%200 "/Game/CustomMaps/UGC2436162648/PushAdvancedPack/MobileSpawns/Plane/Meshes/Parachuting/Backpack/Backpack.Backpack" :Option%201 "/Game/CustomMaps/UGC2436162648/PushAdvancedPack/MobileSpawns/Plane/Meshes/Parachuting/Backpack/Backpack_US.Backpack_US"))
  (Rendering|Material|SetMaterial (Variables|Default|GetBackpack) 0 (Utilities|Select :Index TeamID :Option%200 "/Game/CustomMaps/UGC2436162648/PushAdvancedPack/MobileSpawns/Plane/Meshes/Parachuting/Backpack/M_Backpack_GER.M_Backpack_GER" :Option%201 "/Game/CustomMaps/UGC2436162648/PushAdvancedPack/MobileSpawns/Plane/Meshes/Parachuting/Backpack/M_Backpack_US.M_Backpack_US")))

(event EventBeginPlay
  (bind _pawnowner (Variables|Default|GetPawnOwner))
  (bind _pawnowner_2 (Variables|Default|GetPawnOwner))
  (bind _backpack (Variables|Default|GetBackpack))
  (bind _returnvalue (Transformation|GetSocketTransform _backpack "AttachPoint" "RTS_World"))
  (Networking|SwitchHasAuthority
    (:Authority
      (Actor|SetOwner _pawnowner_2)
      (Utilities|FlowControl|Delay 0.2)
      (bind _returnvalue_2 (Game|SpawnActorfromClass "/Game/CustomMaps/UGC2436162648/PushAdvancedPack/MobileSpawns/Plane/Blueprints/BP_Parachute.BP_Parachute_C" (Math|Transform|MakeTransform (.location _returnvalue) (.rotation _returnvalue) "0.000000,0.000000,0.000000") "AlwaysSpawn" _pawnowner _pawnowner 1e+05 "/Game/CustomMaps/UGC2436162648/PushAdvancedPack/MobileSpawns/Plane/Sounds/parachute_sound.parachute_sound" self 0))
      (Transformation|AttachActorToActor _returnvalue_2 _pawnowner_2 "None" "KeepWorld" "SnapToTarget" "KeepWorld" true)
      (CallFunction|MulticastMesh (Variables|Default|GetTeamID)))))

(fn ConstructionScript)