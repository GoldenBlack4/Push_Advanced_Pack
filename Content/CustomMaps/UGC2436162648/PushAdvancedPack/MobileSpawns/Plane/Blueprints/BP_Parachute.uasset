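; Parachute actor that opens on its owning character, slows the fall and closes on landing.
; The server traces downward each tick, setting fall velocity from clamped ground distance, so descent eases near the ground, and mirrors it through VelocityClient.
; Landing triggers detach, closing animation and delayed destruction, while a failed trace or invalid owner destroys parachute and backpack immediately.
; A repeating timer also removes parachutes whose ground distance stops changing mid-fall.
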(event Custom|VelocityClient
  (params (PawnOwner :type Pawn%20Object%20Reference) (Velocity%20Z :type Float%20%28single-precision%29))
  ;[1 1 1] Tick
  (bind _ascharacter_movement_component (Utilities|CastCharac PawnOwner)
    (:then
      (Variables|/Script/Engine.MovementComponent|SetVelocity _ascharacter_movement_component (Math|Vector|MakeVector 0.0 0.0 Velocity%20Z)))))

(event Custom|OpenAnimation
  (params (PawnOwner :type Pawn%20Object%20Reference))
  ;[1 1 1] Animations
  (Variables|Default|SetPawnOwner PawnOwner)
  (Components|Animation|PlayAnimation (Variables|Default|GetParachute) "/Game/CustomMaps/UGC2436162648/PushAdvancedPack/MobileSpawns/Plane/Meshes/Parachuting/Parachute/Parachute_Anim_Sphere_Opening.Parachute_Anim_Sphere_Opening" false)
  (Transformation|SetActorScale3D "1.000000,1.000000,1.000000")
  (Utilities|FlowControl|Delay 1.5)
  (Components|Animation|PlayAnimation (Variables|Default|GetParachute) "/Game/CustomMaps/UGC2436162648/PushAdvancedPack/MobileSpawns/Plane/Meshes/Parachuting/Parachute/Parachute_Anim_Sphere_Flying.Parachute_Anim_Sphere_Flying" true)
  (Variables|Default|SetParachuteOpened true))

(event Custom|DestroyActor
  ;[1 1 1] Destroy Actor
  (Actor|SetLifeSpan (Variables|Default|GetBackPackRef) 1e+01)
  (Actor|DestroyActor))

(event Custom|ClosingAnimation
  ;[1 1 1] Animations
  (Transformation|DetachFromActor "KeepWorld" "KeepWorld" "KeepWorld")
  (Components|Animation|PlayAnimation (Variables|Default|GetParachute) "/Game/CustomMaps/UGC2436162648/PushAdvancedPack/MobileSpawns/Plane/Meshes/Parachuting/Parachute/Parachute_Anim_Sphere_Closing.Parachute_Anim_Sphere_Closing" false))

(event Custom|CloseParachuteServer
  (bind _pawnowner (Variables|Default|GetPawnOwner))
  ;[1 1 1] Animations
  (CallFunction|ClosingAnimation)
  (if (Actor|ActorHasTag _pawnowner "Backpack")
    (Utilities|Array|RemoveItem (Variables|/Script/Engine.Actor|GetTags _pawnowner) "Backpack"))
  (Utilities|FlowControl|Delay 1e+01)
  (CallFunction|DestroyActor))

(event Custom|ParachuteSound
  ;[1 1 1] Sound
  (Audio|PlaySoundatLocation (Variables|Default|GetParachOpenSound) (Transformation|GetActorLocation) "0, 0, 0" 2.0 1.0 0.0 0 0 0))

(event Custom|DestroyInstantMulticast
  ;[1 1 1] Destroy Actor
  (Actor|DestroyActor (Variables|Default|GetBackPackRef))
  (Actor|DestroyActor))

(event Custom|Timer
  ;[1 1 1] AliveTimer
  (Variables|Default|SetLastDistance (Variables|Default|GetDistance))
  (Utilities|FlowControl|Delay 0.5)
  (if (Math|Boolean|ANDBoolean (== (Variables|Default|GetDistance) (Variables|Default|GetLastDistance)) (Variables|Default|GetIsFalling) (Variables|Default|GetParachuteOpened))
    (Utilities|FlowControl|DoOnce false
      (:Completed
        (CallFunction|ClosingAnimation)
        (Utilities|FlowControl|Delay 2.0)
        (CallFunction|DestroyInstantMulticast)))))

(event EventTick
  (params (DeltaSeconds :type Float%20%28single-precision%29))
  ;[1 1 1] Tick
  (Networking|SwitchHasAuthority
    (:Authority
      (if (Variables|Default|GetParachuteOpened)
        (Utilities|IsValid (Variables|Default|GetPawnOwner)
          (:Is%20Valid
            (bind _ascharacter_movement_component (Utilities|CastCharac (Variables|Default|GetPawnOwner))
              (:then
                (bind _output_get (Variables|Default|SetIsFalling (AI|Components|NavMovement|IsFalling _ascharacter_movement_component)))
                (if _output_get
                  (bind (_outhit _returnvalue) (CallFunction|LineTrace))
                  (if _returnvalue
                    (Variables|Default|SetImpactLocation (.ImpactPoint (Collision|BreakHitResult _outhit)))
                    (Variables|Default|SetDistance (.Distance (Collision|BreakHitResult _outhit)))
                    (Variables|/Script/Engine.MovementComponent|SetVelocity _ascharacter_movement_component (Math|Vector|MakeVector 0.0 0.0 (* (Math|Float|Clamp(Float) (.Distance (Collision|BreakHitResult _outhit)) 1e+02 1.5e+03) -1.0)))
                    (CallFunction|VelocityClient (Variables|Default|GetPawnOwner) (* (Math|Float|Clamp(Float) (.Distance (Collision|BreakHitResult _outhit)) 1e+02 1.5e+03) -1.0))
                    (else
                      (CallFunction|DestroyInstantMulticast :!label _label)))
                  (else
                    (Utilities|FlowControl|DoOnce false
                      (:Completed
                        (Utilities|FlowControl|Delay 0.5)
                        (Variables|Default|SetParachuteOpened false)
                        (CallFunction|CloseParachuteServer))))))
              (:CastFailed
                (goto _label))))
          (:Is%20Not%20Valid
            (goto _label)))))))

(event EventBeginPlay
  (bind _pawnowner (Variables|Default|GetPawnOwner))
  ;[1 1 1] BeginPlay
  (Utilities|FlowControl|Delay 0.2)
  (Actor|SetLifeSpan 6e+01)
  (Networking|SwitchHasAuthority
    (:Authority
      (Actor|SetOwner _pawnowner)
      (CallFunction|ParachuteSound)
      (CallFunction|OpenAnimation _pawnowner)
      (Utilities|Time|SetTimerbyEvent (delegate Custom|Timer) 1.0 true))))

(fn ConstructionScript)

(fn LineTrace
  (bind _pawnowner (Variables|Default|GetPawnOwner))
  (bind _returnvalue (Transformation|GetActorLocation _pawnowner))
  (bind (_x _y _z) (Math|Vector|BreakVector _returnvalue))
  (bind (_outhit _returnvalue_2) (Collision|LineTraceByChannel _returnvalue (Math|Vector|MakeVector _x _y (- _z (Variables|Default|GetLineTraceDistance))) "TraceTypeQuery1" false 0 "ForOneFrame" true "(R=1.000000,G=0.000000,B=0.000000,A=1.000000)" "(R=0.000000,G=1.000000,B=0.000000,A=1.000000)" 999.0))
  (return _outhit _returnvalue_2))