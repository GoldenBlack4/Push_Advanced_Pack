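; A manually placed parachute trigger box that gives backpacks to pawns entering its overlap volume.
; On the server, an overlapping pawn without the Backpack tag gets a BP_Backpack carrying its owner and Pavlov team ID, defaulting to team 1 if the status lookup fails.
; The backpack attaches to any character skeletal mesh with a spine_03 socket, then the pawn's tags are overwritten to prevent repeat grants.
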(event OnComponentBeginOverlap(SpawnParachuteOverlap)
  (params (OverlappedComponent :type Primitive%20Component%20Object%20Reference) (OtherActor :type Actor%20Object%20Reference) (OtherComp :type Primitive%20Component%20Object%20Reference) (OtherBodyIndex :type Integer) (bFromSweep :type Boolean) (SweepResult :type Hit%20Result%20Structure%20%28by%20ref%29))
  ;[1 1 1] Parachute Overlaping Box
  (Networking|SwitchHasAuthority
    (:Authority
      (bind _aspawn (Utilities|Casting|CastToPawn OtherActor))
      (if (not (Actor|ActorHasTag _aspawn "Backpack"))
        (bind (_playerstatus _bsucceeded) (Class|PavlovProxyStatics|GetPavlovPlayerStatusbyPawn _aspawn))
        (bind _ascharacter (Utilities|Casting|CastToCharacter _aspawn))
        (for _array_element (Actor|GetComponentsByClass _ascharacter "/Script/Engine.SkeletalMeshComponent")
          (if (Transformation|DoesSocketExist _array_element "spine_03")
            (bind _returnvalue (Game|SpawnActorfromClass "/Game/CustomMaps/UGC2436162648/PushAdvancedPack/MobileSpawns/Plane/Blueprints/BP_Backpack.BP_Backpack_C" (Math|Transform|MakeTransform (Transformation|GetSocketLocation _array_element "spine_03") "0, 0, 0" "1,1,1") "AlwaysSpawn" 0 (select _bsucceeded (.TeamId (Utilities|Struct|BreakPavlovPlayerStatus _playerstatus)) 1) _aspawn 0))
            (Transformation|AttachComponentToComponent _returnvalue _array_element "spine_03" "SnapToTarget" "SnapToTarget" "KeepWorld" true)
            (Variables|/Script/Engine.Actor|SetTags _aspawn (Variables|Default|GetBackPack))))))))

(fn ConstructionScript)