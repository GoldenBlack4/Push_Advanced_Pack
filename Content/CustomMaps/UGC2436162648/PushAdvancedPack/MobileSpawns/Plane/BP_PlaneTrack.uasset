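; Spline track actor, apparently for the plane mobile spawn, that marks out a configurable number of points along its path.
; The construction script adds evenly spaced text render components from spline start to end and collects them in SplinePoints.
; Each label displays its array index, and OrientToSpline optionally rotates it to the spline direction.
; The event graph holds no active logic.
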(event Collision|EventActorBeginOverlap
  (params (OtherActor :type Actor%20Object%20Reference)))

(event EventTick
  (params (DeltaSeconds :type Float%20%28single-precision%29)))

(fn ConstructionScript
  (Variables|Default|SetNumber%20of%20meshes (Variables|Default|GetNumberOfPoints))
  (if (> (Variables|Default|GetNumber%20of%20meshes) 0)
    (for _index (range 0 (- (Variables|Default|GetNumber%20of%20meshes) 1)) ; Repeat loop for each mesh to add
      (bind _returnvalue (AddComponent|AddTextRenderComponent false (Math|Transform|MakeTransform (Math|Transform|InverseTransformLocation (Transformation|GetActorTransform) (Spline|GetLocationatDistanceAlongSpline (Variables|Default|GetSpline) (* _index (/ (Spline|GetSplineLength (Variables|Default|GetSpline)) (Math|Conversions|ToFloat(Integer) (- (Variables|Default|GetNumber%20of%20meshes) 1)))) "World")))))
      (bind _returnvalue_2 (Utilities|Array|AddUnique (Variables|Default|GetSplinePoints) _returnvalue))
      (Rendering|Components|TextRender|SetText _returnvalue (Utilities|Text|ToText(Integer) _returnvalue_2))
      (if (Variables|Default|GetOrient%20to%20spline)
        (Transformation|SetWorldRotation _returnvalue (Spline|GetRotationatDistanceAlongSpline (Variables|Default|GetSpline) (* _index (/ (Spline|GetSplineLength (Variables|Default|GetSpline)) (Math|Conversions|ToFloat(Integer) (- (Variables|Default|GetNumber%20of%20meshes) 1)))) "World") false false) ; Rotate mesh to match direction of spline at its position
      ))))