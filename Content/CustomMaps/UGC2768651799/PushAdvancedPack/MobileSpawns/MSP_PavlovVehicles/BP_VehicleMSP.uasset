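; BP_VehicleMSP is a team-colored mobile spawn point that rides on a wheeled vehicle.
; On the server it polls its box for an untagged vehicle, tags and attaches to it, then each second sets Ready when its capsule is clear and the vehicle nearly stationary.
; Ready's OnRep toggles the widget; clients assign a per-team scene capture texture.
; If the vehicle becomes invalid, it respawns itself at its initial transform.
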(event Custom|SpawningTick
  (bind _capsule (Variables|Default|GetCapsule))
  ;[1 1 1] Logic
  (bind _vehicle (Variables|Default|GetVehicle)
    (:then
      (Variables|Default|SetReady (and (== (+ (Utilities|Array|Length (Class|PrimitiveComponent|GetOverlappingComponents _capsule)) (Utilities|Array|Length (Collision|GetOverlappingActors _capsule 0 :!class /Script/Engine.PrimitiveComponent))) 0) (Math|Vector|Equal(Vector) (Transformation|GetVelocity _vehicle) "0, 0, 0" 2e+01))))
    (:else
      (Utilities|FlowControl|DoOnce false
        (:Completed
          (Game|SpawnActorfromClass "BP_VehicleMSP_C" (Variables|Default|GetInitialTransform) "AlwaysSpawn" 0 (Variables|Default|GetIsTeam0) 0)
          (Utilities|FlowControl|Delay 0.2)
          (Actor|DestroyActor))))))

(event Custom|SetColor
  (params (Index :type Boolean))
  (bind _returnvalue (select Index "(R=0.000000,G=0.400744,B=1.000000,A=1.000000)" "(R=1.000000,G=0.073878,B=0.000000,A=1.000000)"))
  (bind _widget (Variables|Default|GetWidget))
  (Class|WidgetComponent|SetTintColorandOpacity _widget _returnvalue)
  (Class|WidgetComponent|SetBackgroundColor _widget _returnvalue))

(event Custom|AttachToActor
  (params (ParentActor :type Actor%20Object%20Reference))
  (Transformation|AttachActorToActor ParentActor "None" "SnapToTarget" "SnapToTarget" "SnapToTarget" true))

(event Custom|SetHiddenMulticast
  (params (NewTransform :type Transform%20%28by%20ref%29))
  ;[1 1 1] Hide Widget
  (Development|SetHiddeninGame (Variables|Default|GetWidget) (not (Variables|Default|GetReady)) false)
  (Transformation|SetActorTransform NewTransform false true))

(event EventBeginPlay
  (bind _box (Variables|Default|GetBox))
  (bind _overlappingactors (Collision|GetOverlappingActors _box 0 :!class /Script/Engine.PrimitiveComponent))
  (bind _returnvalue (Utilities|Array|Length _overlappingactors))
  (Utilities|FlowControl|Delay 2.0)
  (Networking|SwitchHasAuthority
    (:Authority
      (CallFunction|SetColor (Variables|Default|GetIsTeam0))
      (Utilities|FlowControl|Delay 1.0 :!label _label)
      (if (> _returnvalue 0)
        (bind _aswheeled_vehicle (Utilities|Casting|CastToWheeledVehicle (Utilities|Array|Get(acopy) _overlappingactors (Math|Random|RandomInteger _returnvalue)))
          (:then
            (if (Utilities|Array|ContainsItem (Variables|/Script/Engine.Actor|GetTags _aswheeled_vehicle) "MSP")
              (goto _label)
              (else
                (Utilities|FlowControl|DoOnce false
                  (:Completed
                    (bind _output_get (Variables|Default|SetVehicle _aswheeled_vehicle))
                    (Variables|/Script/Engine.Actor|SetTags _output_get (Variables|Default|GetTag))
                    (CallFunction|AttachtoActor _output_get)
                    (Utilities|Time|SetTimerbyEvent (delegate Custom|SpawningTick) 1.0 true))))))
          (:CastFailed
            (goto _label)))
        (else
          (goto _label))))
    (:Remote
      (Variables|/Script/Engine.SceneCaptureComponent2D|SetTextureTarget (Variables|Default|GetSceneCaptureComponent2D) (select (Variables|Default|GetIsTeam0) (Variables|Default|GetTextureTeam0) (Variables|Default|GetTextureTeam1))))))

(fn ConstructionScript
  (bind _isteam0 (Variables|Default|GetIsTeam0))
  (bind _widget (Variables|Default|GetWidget))
  (bind _returnvalue (select _isteam0 "(R=0.000000,G=0.400744,B=1.000000,A=1.000000)" "(R=1.000000,G=0.073878,B=0.000000,A=1.000000)"))
  (Variables|Default|SetInitialTransform (Transformation|GetActorTransform))
  (Class|WidgetComponent|SetTintColorandOpacity _widget _returnvalue)
  (Class|WidgetComponent|SetBackgroundColor _widget _returnvalue))

(fn OnRepReady
  (CallFunction|SetHiddenMulticast (Transformation|GetActorTransform)))