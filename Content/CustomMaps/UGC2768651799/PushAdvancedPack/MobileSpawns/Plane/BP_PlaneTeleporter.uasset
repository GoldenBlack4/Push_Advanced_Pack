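; Team-specific spawn teleporter for a Pavlov map that moves pawns in its collision volume onto a random same-team BP_Plane.
; On the server it checks game mode and active Push objective, then spawns, waits in five-second retries, or destroys itself.
; Once active, a looping timer scans overlapping pawns, filters by team, queues bots to jump, and teleports them.
; The construction script sets team label text and colour.
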(event Custom|SpawnPlayers
  (bind _teleportercollision (Variables|Default|GetTeleporterCollision))
  (bind _overlappingactors (Collision|GetOverlappingActors _teleportercollision "/Script/Engine.Pawn" :!class /Script/Engine.PrimitiveComponent))
  (bind _planeavailable (CallFunction|PlaneSelection))
  (if _planeavailable
    (if (> (Utilities|Array|Length _overlappingactors) 0)
      (for _array_element _overlappingactors
        (bind _aspawn (Utilities|Casting|CastToPawn _array_element))
        (bind (_playerstatus _bsucceeded) (Class|PavlovProxyStatics|GetPavlovPlayerStatusbyPawn _aspawn))
        (if _bsucceeded
          (Utilities|CanbeTeleported (.TeamId (Utilities|Struct|BreakPavlovPlayerStatus _playerstatus))
            (:Yes
              (if (Pawn|IsPlayerControlled _aspawn) :!label _label
                _
                (else
                  (Default|AddBottoJumpWaitingList (Variables|Default|GetChoosenPlane) _aspawn)))
              (CallFunction|Teleporting _aspawn)))
          (else
            ;[1 0 0] Debug
            (if (Utilities|String|StartsWith (Utilities|GetDisplayName _aspawn) "PlayerChara")
              (goto _label))))))))

(event EventBeginPlay
  (Networking|SwitchHasAuthority
    (:Authority
      (Utilities|PushMacro :!label _label
        (:Spawn
          (Variables|Default|SetWait false)
          (if (Variables|Default|GetWait) :!label _label_2
            (Utilities|FlowControl|Delay 5.0)
            (goto _label)
            (else
              (Utilities|FlowControl|DoOnce false
                (:Completed
                  (Utilities|FlowControl|Delay 0.5)
                  (Utilities|Time|SetTimerbyEvent (delegate Custom|SpawnPlayers) 0.2 true))))))
        (:Destroy
          (Actor|DestroyActor))
        (:Wait
          (Variables|Default|SetWait true)
          (goto _label_2))))))

(fn ConstructionScript
  (bind _teamtext (Variables|Default|GetTeamText))
  (Rendering|Components|TextRender|SetText _teamtext (select (Variables|Default|GetIsTeam0) (Utilities|Text|FormatText "Team 0") (Utilities|Text|FormatText "Team 1")))
  (Rendering|Components|TextRender|SetTextRenderColor _teamtext (select (Variables|Default|GetIsTeam0) (Math|Color|MakeColor 255 0 0) (Math|Color|MakeColor 0 0 255))))

(fn PlaneSelection
  (bind _availableplanes (Variables|Default|GetAvailablePlanes))
  (bind _outactors (Actor|GetAllActorsOfClass "/Game/CustomMaps/UGC2768651799/PushAdvancedPack/MobileSpawns/Plane/BP_Plane.BP_Plane_C"))
  (Utilities|Array|Clear (Variables|Default|GetAvailablePlanes))
  (if (> (Utilities|Array|Length _outactors) 0)
    (for _array_element _outactors
      (if (Math|Boolean|Equal(Boolean) (Variables|/Game/CustomMaps/UGC2768651799/PushAdvancedPack/MobileSpawns/Plane/BP_Plane.BP_Plane_C|GetIsTeam0 _array_element) (Variables|Default|GetIsTeam0))
        (Utilities|Array|Add (Variables|Default|GetAvailablePlanes) _array_element)))
    (Variables|Default|SetChoosenPlane (Utilities|Array|Get(acopy) _availableplanes (Math|Random|RandomInteger (Utilities|Array|Length _availableplanes))))
    (return true)
    (else
      (return false))))

(fn Teleporting
  (params (Pawn :type Pawn%20Object%20Reference))
  (Transformation|Teleport Pawn (select (Variables|Default|GetIsABot) (Transformation|GetWorldLocation (Variables|/Game/CustomMaps/UGC2768651799/PushAdvancedPack/MobileSpawns/Plane/BP_Plane.BP_Plane_C|GetBotsTeleportLocation (Variables|Default|GetChoosenPlane))) (Transformation|GetWorldLocation (Variables|/Game/CustomMaps/UGC2768651799/PushAdvancedPack/MobileSpawns/Plane/BP_Plane.BP_Plane_C|GetPlayersTeleportLocation (Variables|Default|GetChoosenPlane)))) "0, 0, 0")
  (return))