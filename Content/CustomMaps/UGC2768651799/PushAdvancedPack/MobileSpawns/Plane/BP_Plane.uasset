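; Troop transport plane that flies a spline track and drops players and bots by parachute.
; A multicast timeline moves it; reaching set spline points toggles the replicated LightGreen, whose RepNotify recolors the jump light and animates the doors.
; While green, a looping timer sends queued bots to the eject point by AI move, teleporting them on failure.
; The server attaches team-tagged BP_Backpack parachutes to pawns entering the overlap box.
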(event OnComponentBeginOverlap(SpawnParachuteOverlap)
  (params (OverlappedComponent :type Primitive%20Component%20Object%20Reference) (OtherActor :type Actor%20Object%20Reference) (OtherComp :type Primitive%20Component%20Object%20Reference) (OtherBodyIndex :type Integer) (bFromSweep :type Boolean) (SweepResult :type Hit%20Result%20Structure%20%28by%20ref%29))
  ;[1 1 1] Parachute Overlaping Box
  (Networking|SwitchHasAuthority
    (:Authority
      (bind _aspawn (Utilities|Casting|CastToPawn OtherActor))
      (if (not (Actor|ActorHasTag _aspawn "Backpack"))
        (bind (_playerstatus _bsucceeded) (Class|PavlovProxyStatics|GetPavlovPlayerStatusbyPawn _aspawn))
        (bind _ascharacter (Utilities|Casting|CastToCharacter _aspawn))
        (for _array_element (Actor|GetComponentsByClass _ascharacter "/Script/Engine.SkeletalMeshComponent")
          (if (Transformation|DoesSocketExist _array_element "spine_03")
            (bind _returnvalue (Game|SpawnActorfromClass "/Game/CustomMaps/UGC2768651799/PushAdvancedPack/MobileSpawns/Plane/Blueprints/BP_Backpack.BP_Backpack_C" (Math|Transform|MakeTransform (Transformation|GetSocketLocation _array_element "spine_03") "0, 0, 0" "1,1,1") "AlwaysSpawn" 0 (select _bsucceeded (.TeamId (Utilities|Struct|BreakPavlovPlayerStatus _playerstatus)) 1) _aspawn 0))
            (Transformation|AttachComponentToComponent _returnvalue _array_element "spine_03" "SnapToTarget" "SnapToTarget" "KeepWorld" true)
            (Variables|/Script/Engine.Actor|SetTags _aspawn (Variables|Default|GetBackPack))))))))

(event Custom|Doors
  (bind _door_2_openrelrotation (Variables|Default|GetDoor_2_OpenRelRotation))
  (bind _door_1_openrelrotation (Variables|Default|GetDoor_1_OpenRelRotation))
  ;[1 1 1] Doors
  (Utilities|FlowControl|Delay 1.0)
  (if (Variables|Default|GetLightGreen)
    (bind _alpha (Timeline|Timeline_0 Reverse)
      (:Update
        (Transformation|SetRelativeRotation (Variables|Default|GetDoor_2) (Math|Interpolation|RInterpTo (Variables|Default|GetDoor_2_OpenRelRotation) (Math|Rotator|MakeRotator (+ (.roll _door_2_openrelrotation) (Variables|Doors_Rotation|GetDoor_2_Roll)) (+ (.pitch _door_2_openrelrotation) (Variables|Doors_Rotation|GetDoor_2_Pitch)) (+ (.yaw _door_2_openrelrotation) (Variables|Doors_Rotation|GetDoor_2_Yaw))) _alpha 1.0) false true)
        (Transformation|SetRelativeRotation (Variables|Default|GetDoor_1) (Math|Interpolation|RInterpTo (Variables|Default|GetDoor_1_OpenRelRotation) (Math|Rotator|MakeRotator (+ (.roll _door_1_openrelrotation) (Variables|Doors_Rotation|GetDoor_1_Roll)) (+ (.pitch _door_1_openrelrotation) (Variables|Doors_Rotation|GetDoor_1_Pitch)) (+ (.yaw _door_1_openrelrotation) (Variables|Doors_Rotation|GetDoor_1_Yaw))) _alpha 1.0) false true)))
    (else
      (Timeline|Timeline_0 Play))))

(event Custom|EjectBots
  (bind _waitinglist (Variables|Default|GetWaitingList))
  (bind _botsejectlocation (Variables|Default|GetBotsEjectLocation))
  (bind _returnvalue (Transformation|GetWorldLocation _botsejectlocation))
  (bind _output (Utilities|Array|Get(acopy) _waitinglist))
  ;[1 1 1] Force Bots to Jump
  (if (> (Utilities|Array|Length _waitinglist) 0)
    (if (Variables|Default|GetLightGreen)
      (AI|AIMoveTo _output _returnvalue 0 1.0 false
        (:OnSuccess
          (Utilities|Array|RemoveItem (Variables|Default|GetWaitingList) _output :!label _label))
        (:OnFail
          (bind _returnvalue_2 (Transformation|Teleport _output _returnvalue "0, 0, 0"))
          (if _returnvalue_2
            (goto _label)))))))

(event Custom|MovePlaneMulticast
  (bind _trackreference (Variables|Default|GetTrackReference))
  (bind _plane (Variables|Default|GetPlane))
  (bind _trackreference_2 (Variables|Default|GetTrackReference))
  (bind _returnvalue (Transformation|GetWorldTransform _plane))
  (bind _spline (Variables|/Game/CustomMaps/UGC2768651799/PushAdvancedPack/MobileSpawns/Plane/BP_PlaneTrack.BP_PlaneTrack_C|GetSpline _trackreference_2))
  ;[0.4656 0.3575 1] Plane and Spline Logic
  (bind _alpha (Timeline|PlaneMover Play)
    (:Update
      (Variables|Default|SetAlpha _alpha)
      (Transformation|SetActorLocationAndRotation (Math|Interpolation|VInterpTo (.location _returnvalue) (Spline|GetLocationatDistanceAlongSpline _spline (Math|Float|Lerp 0.0 (Spline|GetSplineLength _spline) (Variables|Default|GetAlpha)) "World") (Variables|Default|GetAlpha) 1.0) (Math|Interpolation|RInterpTo (.rotation _returnvalue) (Spline|GetRotationatDistanceAlongSpline _spline (Math|Float|Lerp 0.0 (Spline|GetSplineLength _spline) (Variables|Default|GetAlpha)) "World") (Variables|Default|GetAlpha) 1.0) false true)
      (if (Variables|Default|GetNoDoorsClosing)
        (Utilities|FlowControl|DoOnce false :!label _label
          (:Completed
            (CallFunction|SetGreenLight)
            (goto _label_2 Reset)))
        (elif (Math|Vector|Equal(Vector) (Transformation|GetWorldLocation (Utilities|Array|Get(acopy) (Variables|/Game/CustomMaps/UGC2768651799/PushAdvancedPack/MobileSpawns/Plane/BP_PlaneTrack.BP_PlaneTrack_C|GetSplinePoints _trackreference) (Variables|Default|GetDoorsOpenPoint))) (.location _returnvalue) 1e+01)
          (goto _label)
          (elif (Math|Vector|Equal(Vector) (.location _returnvalue) (Transformation|GetWorldLocation (Utilities|Array|Get(acopy) (Variables|/Game/CustomMaps/UGC2768651799/PushAdvancedPack/MobileSpawns/Plane/BP_PlaneTrack.BP_PlaneTrack_C|GetSplinePoints _trackreference) (Variables|Default|GetDoorsClosePoint))) 1e+01)
            (Utilities|FlowControl|DoOnce false :!label _label_2
              (:Completed
                (CallFunction|SetRedLight)
                (goto _label Reset)))))))))

(event Custom|AddBotToJumpWaitingList
  (params (Pawn :type Pawn%20Object%20Reference%20%28by%20ref%29))
  ;[1 1 1] Force Bots to Jump
  (Utilities|Array|Add (Variables|Default|GetWaitingList) Pawn))

(event Custom|SetGreenLight
  ;[0.4656 0.3575 1] Plane and Spline Logic
  (Variables|Default|SetLightGreen true))

(event Custom|SetRedLight
  ;[0.4656 0.3575 1] Plane and Spline Logic
  (Variables|Default|SetLightGreen false))

(event Custom|SetTimerBotsEjecting
  ;[1 1 1] Force Bots to Jump
  (Utilities|Time|SetTimerbyEvent (delegate Custom|EjectBots) 1.0 true))

(event EventBeginPlay
  ;[1 1 1] BeginPlay
  (Utilities|FlowControl|Delay 1.0)
  (Components|Timeline|SetPlayRate (Variables|Default|GetPlaneMover) (/ 1.0 (Variables|Default|GetPlaneSpeed)))
  (Components|Timeline|SetNewTime (Variables|Default|GetPlaneMover) (Variables|Default|GetPlaneStartOffset))
  (Networking|SwitchHasAuthority
    (:Authority
      (CallFunction|MovePlaneMulticast)
      (CallFunction|SetTimerBotsEjecting)
      (Variables|Default|SetLightGreen (Variables|Default|GetLightGreen))
      (Collision|SetCollisionEnabled (Variables|Default|GetDoor_1) "NoCollision"))
    (:Remote
      (Utilities|FlowControl|Delay 2.0)
      (Variables|Default|SetLightGreen (Variables|Default|GetLightGreen)))))

(event EventTick
  (params (DeltaSeconds :type Float%20%28single-precision%29))
  ;[1 1 1] Tick
  (Transformation|AddLocalRotation (Variables|Default|GetPropeller_1) "0, 0,10.000000" false false))

(fn ConstructionScript
  (bind _trackreference (Variables|Default|GetTrackReference))
  (bind _spline (Variables|/Game/CustomMaps/UGC2768651799/PushAdvancedPack/MobileSpawns/Plane/BP_PlaneTrack.BP_PlaneTrack_C|GetSpline _trackreference))
  (Variables|Default|SetDoor_1_OpenRelRotation (Variables|/Script/Engine.SceneComponent|GetRelativeRotation (Variables|Default|GetDoor_1)))
  (Variables|Default|SetDoor_2_OpenRelRotation (Variables|/Script/Engine.SceneComponent|GetRelativeRotation (Variables|Default|GetDoor_2)))
  (Utilities|IsValid _trackreference
    (:Is%20Valid
      (Transformation|SetActorLocationAndRotation (Spline|GetLocationatSplinePoint _spline 0 "World") (Spline|GetRotationatSplinePoint _spline 0 "World") false true))))

(fn ParachuteLocation
  (bind _returnvalue (Game|GetPlayerCameraManager 0))
  (bind _returnvalue_2 (Utilities|Time|GetWorldDeltaSeconds))
  (bind _parachute_speed (Variables|Default|GetParachute%20Speed))
  (bind _stopping_scalar (Variables|Default|GetStopping%20Scalar))
  (bind _returnvalue_3 (Math|Float|Clamp(Float) _stopping_scalar 0.5))
  (bind _rootcomponent (Variables|/Script/Engine.Actor|GetRootComponent _returnvalue))
  (bind _returnvalue_4 (Math|Vector|GetForwardVector _rootcomponent))
  (bind _returnvalue_5 (* _returnvalue_3 _parachute_speed))
  (bind _returnvalue_6 (* _returnvalue_4 _returnvalue_5))
  (bind _returnvalue_7 (* _returnvalue_6 _returnvalue_2))
  (return (Math|Vector|MakeVector (.x _returnvalue_7) (.y _returnvalue_7) (* (* (Math|Float|MapRangeClamped (Variables|Default|GetStopping%20Scalar) 0.0 1.0 1.0 0.65) (Variables|Default|GetParachuteGravity)) (Utilities|Time|GetWorldDeltaSeconds)))))

(fn OnRepLightGreen
  (bind _pointlight (Variables|Default|GetPointLight))
  (if (Variables|Default|GetLightGreen)
    (Rendering|Components|Light|SetLightColor _pointlight "(R=0.042311,G=1.000000,B=0.000000,A=1.000000)" true)
    (else
      (Rendering|Components|Light|SetLightColor _pointlight "(R=1.000000,G=0.007499,B=0.000000,A=1.000000)" true)))
  (CallFunction|Doors))