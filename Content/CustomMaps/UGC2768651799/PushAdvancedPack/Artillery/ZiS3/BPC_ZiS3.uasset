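; BPC_ZiS3 is a child Blueprint for the ZiS-3 artillery gun in a Pavlov custom map pack.
; On BeginPlay it runs the parent logic, waits briefly, then attaches PavlovFire and the ATLRWheel and ATUDWheel components to ATRail, keeping their world transforms.
; The construction script only calls the parent, and the file defines no other active logic.
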(event EventBeginPlay
  (|CallParentFunction)
  (Utilities|FlowControl|Delay 1.0)
  (Transformation|AttachComponentToComponent (Variables|Default|GetPavlov_Fire) (Variables|Default|GetAT_Rail) "None" "KeepWorld" "KeepWorld" "KeepWorld" true)
  (Transformation|AttachComponentToComponent (Variables|Default|GetAT_LRWheel) (Variables|Default|GetAT_Rail) "None" "KeepWorld" "KeepWorld" "KeepWorld" true)
  (Transformation|AttachComponentToComponent (Variables|Default|GetAT_UDWheel) (Variables|Default|GetAT_Rail) "None" "KeepWorld" "KeepWorld" "KeepWorld" true))

(event Collision|EventActorBeginOverlap
  (params (OtherActor :type Actor%20Object%20Reference)))

(event EventTick
  (params (DeltaSeconds :type Float%20%28single-precision%29)))

(fn ConstructionScript
  (|CallParentFunction))