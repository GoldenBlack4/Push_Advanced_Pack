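; Hafthohlladung sticky charge that attaches to a hit component and explodes after a delay if armed.
; On BeginPlay the server runs a one-shot Explode from the Hit variable and replicates the armed or capped mesh.
; Detonation damages actors overlapping OuterRadius, deals heavy extra damage to the hit actor, multicasts effects and destroys the charge.
; A lifespan slightly beyond the fuse cleans up unarmed charges.
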(event Custom|FX_Multicast
  (params (Location :type Vector))
  (Effects|SpawnEmitteratLocation (Variables|Default|GetFireEmitter) Location "0, 0, 0" "3.000000,3.000000,3.000000")
  (Audio|PlaySoundatLocation (Variables|Default|GetBulletExplosion) Location "0, 0, 0" 1.0 1.0 0.0 0 0 0)
  (Audio|PlaySoundatLocation (Variables|Default|GetBulletDistantExplosion) Location "0, 0, 0" 1.0 1.0 0.0 0 0 0))

(event Custom|Explode
  (params (Hit :type Hit%20Result%20Structure%20%28by%20ref%29))
  (bind (_bblockinghit _binitialoverlap _time _distance _location _impactpoint _normal _impactnormal _physmat _hitactor _hitcomponent) (Collision|BreakHitResult Hit))
  (Networking|SwitchHasAuthority
    (:Authority
      (Utilities|FlowControl|DoOnce false
        (:Completed
          (CallFunction|ReplicateAttach _hitcomponent)
          (Variables|Default|SetHitComp _hitcomponent)
          (Variables|Default|SetHitActor _hitactor)
          (Utilities|FlowControl|Delay (Variables|Default|GetExplosionDelay))
          (if (Variables|Default|GetArmed)
            (for _array_element (Collision|GetOverlappingActors (Variables|Default|GetOuterRadius) 0 :!class /Script/Engine.PrimitiveComponent)
              (Game|Damage|ApplyDamage _array_element 9e+01 (Game|GetInstigatorController) self "/Game/CustomMaps/UGC2768651799/PushAdvancedPack/Artillery/Common/Blueprints/DamageType_Mine.DamageType_Mine_C"))
            (Game|Damage|ApplyDamage _hitactor 1e+03 (Game|GetInstigatorController) self "/Game/CustomMaps/UGC2768651799/PushAdvancedPack/Artillery/Common/Blueprints/DamageType_Mine.DamageType_Mine_C")
            (CallFunction|FXMulticast (Transformation|GetActorLocation))
            (Utilities|FlowControl|Delay 0.1)
            (Actor|DestroyActor)))))))

(event Custom|ReplicateAttach
  (params (Parent :type Scene%20Component%20Object%20Reference))
  (Transformation|AttachComponentToComponent Parent "None" "KeepWorld" "KeepWorld" "KeepWorld" true))

(event Custom|ReplicateMeshState
  (params (Condition :type Boolean))
  (bind _mesh (Variables|Default|GetMesh))
  (if Condition
    (Components|StaticMesh|SetStaticMesh _mesh "/Game/CustomMaps/UGC2768651799/PushAdvancedPack/StickyGrenades/Hafthohlladung/Meshes/hafthohlladung.hafthohlladung")
    (else
      (Components|StaticMesh|SetStaticMesh _mesh "/Game/CustomMaps/UGC2768651799/PushAdvancedPack/StickyGrenades/Hafthohlladung/Meshes/hafthohlladung_cap.hafthohlladung_cap"))))

(event EventBeginPlay
  (Utilities|FlowControl|Delay 0.2)
  (Actor|SetLifeSpan (+ (Variables|Default|GetExplosionDelay) 5.0))
  (Networking|SwitchHasAuthority
    (:Authority
      (CallFunction|Explode (Variables|Default|GetHit))
      (CallFunction|ReplicateMeshState (Variables|Default|GetArmed)))))

(fn ConstructionScript)