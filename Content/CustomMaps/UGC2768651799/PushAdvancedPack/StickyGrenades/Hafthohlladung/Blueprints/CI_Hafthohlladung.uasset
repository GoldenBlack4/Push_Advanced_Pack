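; Inventory item for the Hafthohlladung sticky charge, which can be armed and stuck to vehicles or metal surfaces.
; Use arms it with a pin sound, and replicated Armed swaps the capped mesh.
; Pickup starts a looping downward trace that, outside inventory, matches actor name prefixes or metal physical materials, then spawns the grenade actor there and destroys the item.
; Dropped items still in the world despawn after a delay.
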(event Custom|AttachSound
  (Audio|PlaySoundatLocation "/Game/CustomMaps/UGC2768651799/PushAdvancedPack/StickyGrenades/Sound/MetalHit.MetalHit" (Transformation|GetActorLocation) "0, 0, 0" 1.0 1.0 0.0 "/Game/CustomMaps/UGC2768651799/PushAdvancedPack/StickyGrenades/Sound/A_Grenade.A_Grenade" 0 0))

(event Custom|LineTrace
  (bind _returnvalue (Transformation|GetActorLocation))
  ;[1 1 1] Linetrace Client
  (bind _returnvalue_2 (Class|PavlovCustomItem|GetItemState))
  (if (not (Utilities|Enum|Equal(Enum) _returnvalue_2 "InInventory"))
    (bind (_outhit _returnvalue_3) (Collision|LineTraceByChannel _returnvalue (+ _returnvalue (* (Math|Vector|GetUpVector (Transformation|GetActorRotation)) -5e+01)) "TraceTypeQuery1" false 0 "Persistent"))
    (if _returnvalue_3
      (Variables|Default|SetHit _outhit)
      (if (Math|Boolean|ORBoolean (Utilities|String|StartsWith (Utilities|GetDisplayName (.HitActor (Collision|BreakHitResult _outhit))) "Veh") (Utilities|String|StartsWith (Utilities|GetDisplayName (.HitActor (Collision|BreakHitResult _outhit))) "BPC_") (Utilities|String|StartsWith (Utilities|GetDisplayName (.HitActor (Collision|BreakHitResult _outhit))) "BPM_") (Utilities|String|StartsWith (Utilities|GetDisplayName (.HitActor (Collision|BreakHitResult _outhit))) "Tank") (Utilities|String|Contains (Utilities|GetDisplayName (.PhysMat (Collision|BreakHitResult _outhit))) "metal"))
        (Utilities|Time|ClearandInvalidateTimerbyHandle (Variables|Default|GetLineTraceTimer))
        (Utilities|FlowControl|DoOnce false
          (:Completed
            (CallFunction|SpawnAttached (.ImpactPoint (Collision|BreakHitResult _outhit)) (Math|Rotator|MakeRotfromZ (.ImpactNormal (Collision|BreakHitResult _outhit))) (Variables|Default|GetHit))))))))

(event Custom|SetArmed
  (Variables|Default|SetArmed true)
  (CallFunction|ArmedSound))

(event Custom|SpawnAttached
  (params (Spawn%20Transform%20Location :type Vector) (Spawn%20Transform%20Rotation :type Rotator) (Hit :type Hit%20Result%20Structure))
  (bind _pawnowner (Variables|Default|GetPawnOwner))
  ;[1 1 1] Linetrace Client
  (Game|SpawnActorfromClass "/Game/CustomMaps/UGC2768651799/PushAdvancedPack/StickyGrenades/Hafthohlladung/Blueprints/Grenade_Hafthohlladung.Grenade_Hafthohlladung_C" (Math|Transform|MakeTransform Spawn%20Transform%20Location Spawn%20Transform%20Rotation "1,1,1") "AlwaysSpawn" _pawnowner Hit 5.0 (Variables|Default|GetArmed) _pawnowner)
  (CallFunction|AttachSound)
  (Utilities|FlowControl|Delay 0.1)
  (Actor|DestroyActor))

(event Custom|ArmedSound
  (Audio|PlaySoundatLocation "/Game/CustomMaps/UGC2768651799/PushAdvancedPack/StickyGrenades/Sound/GrenadePin_Cue.GrenadePin_Cue" (Transformation|GetActorLocation) "0, 0, 0" 1.0 1.0 0.0 "/Game/CustomMaps/UGC2768651799/PushAdvancedPack/StickyGrenades/Sound/A_Grenade.A_Grenade" 0 0))

(event Custom|SetOwnerServer
  (params (PawnOwner :type Pawn%20Object%20Reference))
  (Variables|Default|SetPawnOwner PawnOwner))

(event Custom|PickupClient
  ;[1 1 1] Linetrace Client
  (bind _returnvalue (Utilities|Time|SetTimerbyEvent (delegate Custom|LineTrace) 0.05 true))
  (Variables|Default|SetLineTraceTimer _returnvalue))

(event EventOnUse
  (Utilities|FlowControl|DoOnce false
    (:Completed
      (CallFunction|SetArmed))))

(event EventOnDrop
  (bind _returnvalue (Class|PavlovCustomItem|GetItemState))
  (if (Utilities|Enum|Equal(Enum) _returnvalue "InWorld")
    (Utilities|FlowControl|Delay 25.0)
    (bind _returnvalue_2 (Class|PavlovCustomItem|GetItemState))
    (if (Utilities|Enum|Equal(Enum) _returnvalue_2 "InWorld")
      (Actor|DestroyActor))))

(event EventOnPickup
  (params (Pawn :type Pawn%20Object%20Reference) (bDominant :type Boolean))
  (CallFunction|PickupClient)
  (CallFunction|SetOwnerServer Pawn))

(fn ConstructionScript)

(fn OnRepArmed
  (bind _mesh (Variables|Default|GetMesh))
  (if (Variables|Default|GetArmed)
    (Components|StaticMesh|SetStaticMesh _mesh "/Game/CustomMaps/UGC2768651799/PushAdvancedPack/StickyGrenades/Hafthohlladung/Meshes/hafthohlladung.hafthohlladung")
    (else
      (Components|StaticMesh|SetStaticMesh _mesh "/Game/CustomMaps/UGC2768651799/PushAdvancedPack/StickyGrenades/Hafthohlladung/Meshes/hafthohlladung_cap.hafthohlladung_cap"))))