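; Carryable Gammon Bomb item that the player arms on use and releases to become a grenade.
; First use arms it on the server and plays the pin sound, and the replicated Armed state updates the mesh.
; When released armed, the server spawns Grenade_GammonBomb with the item's transform, velocity and instigator, then destroys the item.
; When dropped unarmed, it destroys itself after a delay if still in the world.
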(event Custom|OnPickUp_Server
  (params (OwnerPawn :type Pawn%20Object%20Reference))
  (Variables|Default|SetOwnerPawn OwnerPawn))

(event Custom|OnDrop_Server
  (params (SpawnTransform :type Transform) (Velocity :type Vector) (Instigator :type Pawn%20Object%20Reference))
  (Game|SpawnActorfromClass "/Game/CustomMaps/UGC2768651799/PushAdvancedPack/StickyGrenades/GammonBomb/Blueprints/Grenade_GammonBomb.Grenade_GammonBomb_C" SpawnTransform "AlwaysSpawn" (Variables|Default|GetOwnerPawn) Velocity (Variables|Default|GetArmed) Instigator)
  (Utilities|FlowControl|Delay 0.05)
  (Actor|DestroyActor))

(event Custom|OnUse_Server
  (Variables|Default|SetArmed true)
  (CallFunction|PlaySoundFX))

(event Custom|PlaySoundFX
  (Audio|PlaySoundatLocation "/Game/CustomMaps/UGC2768651799/PushAdvancedPack/StickyGrenades/Sound/GrenadePin_Cue.GrenadePin_Cue" (Transformation|GetActorLocation) "0, 0, 0" 1.0 1.0 0.0 "/Game/CustomMaps/UGC2768651799/PushAdvancedPack/StickyGrenades/Sound/A_Grenade.A_Grenade" 0 0))

(event EventOnDrop
  (bind _mesh (Variables|Default|GetMesh))
  (bind _returnvalue (Class|PavlovCustomItem|GetItemState))
  (if (not (Utilities|Enum|Equal(Enum) _returnvalue "InInventory"))
    (if (Variables|Default|GetArmed)
      (Utilities|FlowControl|Delay 0.05)
      (CallFunction|OnDropServer (Transformation|GetWorldTransform _mesh) (Transformation|GetComponentVelocity _mesh) (Variables|Default|GetOwnerPawn))
      (else
        (bind _returnvalue_2 (Class|PavlovCustomItem|GetItemState))
        (if (Utilities|Enum|Equal(Enum) _returnvalue_2 "InWorld")
          (Utilities|FlowControl|Delay 25.0)
          (bind _returnvalue_3 (Class|PavlovCustomItem|GetItemState))
          (if (Utilities|Enum|Equal(Enum) _returnvalue_3 "InWorld")
            (Actor|DestroyActor)))))))

(event EventOnUse
  (Utilities|FlowControl|DoOnce false
    (:Completed
      (if (not (Variables|Default|GetArmed))
        (CallFunction|OnUseServer)))))

(event EventOnPickup
  (params (Pawn :type Pawn%20Object%20Reference) (bDominant :type Boolean))
  (CallFunction|OnPickUpServer Pawn))

(fn ConstructionScript)

(fn OnRepArmed
  (if (Variables|Default|GetArmed)
    (Components|StaticMesh|SetStaticMesh (Variables|Default|GetMesh) "/Game/CustomMaps/UGC2768651799/PushAdvancedPack/StickyGrenades/GammonBomb/Meshes/GammonBomb.GammonBomb")))