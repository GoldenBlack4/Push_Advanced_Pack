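; Parent Blueprint for a placeable artillery construction site that players build with the engineer tool's hammer.
; On authority, each debounced hammer overlap adds health, and the site destroys itself if unfinished after its lifespan or when the round ends.
; The HealthFull RepNotify sets overlap collision while unbuilt; once full, it swaps to a waiting material, waits until no pawns overlap, then spawns a non-respawning artillery spawner and removes itself.
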(event OnComponentBeginOverlap(Mesh)
  (params (OverlappedComponent :type Primitive%20Component%20Object%20Reference) (OtherActor :type Actor%20Object%20Reference) (OtherComp :type Primitive%20Component%20Object%20Reference) (OtherBodyIndex :type Integer) (bFromSweep :type Boolean) (SweepResult :type Hit%20Result%20Structure%20%28by%20ref%29))
  (Networking|SwitchHasAuthority
    (:Authority
      (if (not (Variables|Default|GetHealthFull))
        (bind _asci_engineer_tool (Utilities|Casting|CastToCI_EngineerTool OtherActor))
        (if (== (Variables|/Game/CustomMaps/UGC2768651799/PushAdvancedPack/ClassTools/Tools/Blueprints/CI_EngineerTool.CI_EngineerTool_C|GetHammerCollision _asci_engineer_tool) OtherComp)
          (Utilities|FlowControl|DoOnce false
            (:Completed
              (bind _output_get (Variables|Default|SetHealth (+ (Variables|Default|GetHealth) 1e+01)))
              (CallFunction|RepairSound (Transformation|GetWorldLocation (Variables|/Game/CustomMaps/UGC2768651799/PushAdvancedPack/ClassTools/Tools/Blueprints/CI_EngineerTool.CI_EngineerTool_C|GetHammerCollision _asci_engineer_tool)))
              (Variables|Default|SetHealthFull (>= _output_get (Variables|Default|GetMaxHealth))))))))))

(event OnComponentEndOverlap(Mesh)
  (params (OverlappedComponent :type Primitive%20Component%20Object%20Reference) (OtherActor :type Actor%20Object%20Reference) (OtherComp :type Primitive%20Component%20Object%20Reference) (OtherBodyIndex :type Integer))
  (Networking|SwitchHasAuthority
    (:Authority
      (bind _asci_engineer_tool (Utilities|Casting|CastToCI_EngineerTool OtherActor))
      (Utilities|IsValid (Variables|/Game/CustomMaps/UGC2768651799/PushAdvancedPack/ClassTools/Tools/Blueprints/CI_EngineerTool.CI_EngineerTool_C|GetHammerCollision _asci_engineer_tool)
        (:Is%20Valid
          (Utilities|FlowControl|Delay 0.2)
          (Utilities|FlowControl|DoOnce false) ; enters at Reset
        )))))

(event Custom|SpawnArtillery
  (if (> (Utilities|Array|Length (Collision|GetOverlappingActors (Variables|Default|GetMesh) "/Script/Engine.Pawn" :!class /Script/Engine.PrimitiveComponent)) 0) :!label _label
    (Utilities|FlowControl|Delay 1.0)
    (goto _label)
    (else
      (Utilities|FlowControl|DoOnce false
        (:Completed
          (bind _returnvalue (Game|SpawnActorfromClass "/Game/CustomMaps/UGC2768651799/PushAdvancedPack/Artillery/SPAWNER_Artillery.SPAWNER_Artillery_C" (Transformation|GetActorTransform) "AlwaysSpawn" 0 (Variables|Default|GetArtilleryToSpawn) false 0.2 3e+01 true false false -1 5e+02 "/Game/PyroParticlePack/Particles/PPP_Fire_02.PPP_Fire_02" "/Game/CustomMaps/UGC2768651799/PushAdvancedPack/Artillery/Common/Sound/Fire_Cue.Fire_Cue" "/Game/CustomMaps/UGC2768651799/PushAdvancedPack/Artillery/Common/Sound/trapclose_sound.trapclose_sound" "/Game/CustomMaps/UGC2768651799/PushAdvancedPack/Artillery/Common/Sound/shellloading_sound.shellloading_sound" true false false 1.0 0))
          (Variables|/Script/Engine.Actor|SetTags _returnvalue (Variables|Actor|GetTags))
          (Utilities|FlowControl|Delay 0.2)
          (Actor|DestroyActor))))))

(event Custom|Set%20Collisions
  (bind _mesh (Variables|Default|GetMesh))
  (Collision|SetCollisionResponsetoAllChannels _mesh "ECR_Overlap")
  (Collision|SetCollisionResponsetoChannel _mesh "ECC_Visibility" "ECR_Block"))

(event Custom|SetWaitingMaterial
  (Rendering|Material|SetMaterial (Variables|Default|GetMesh) 0 (Variables|Default|GetWaitingMaterial)))

(event Custom|RepairSound
  (params (Location :type Vector))
  (Audio|PlaySoundatLocation "/Game/CustomMaps/UGC2768651799/PushAdvancedPack/ClassTools/Tools/Sounds/S_WoodHit.S_WoodHit" Location "0, 0, 0" 1.0 1.0 0.0 0 0 0))

(event Custom|PushEndRoundCheck
  (bind _returnvalue (Class|PavlovLibrary|GetGameLogic))
  (Utilities|IsValid _returnvalue
    (:Is%20Valid
      (switch Utilities|FlowControl|Switch|SwitchonEPavlovRoundState (Class|PavlovGameLogic|GetRoundState _returnvalue)
        (:Ended
          (Actor|DestroyActor))))))

(event EventBeginPlay
  (Networking|SwitchHasAuthority
    (:Authority
      (Utilities|FlowControl|Delay 0.2)
      (Utilities|Time|SetTimerbyEvent (delegate Custom|PushEndRoundCheck) 3.0 true)
      (Variables|Default|SetHealthFull false)
      (Utilities|FlowControl|Delay (Variables|Default|GetLifeSpanUnconstructed))
      (if (not (Variables|Default|GetHealthFull))
        (Actor|DestroyActor)))))

(fn ConstructionScript
  (Components|StaticMesh|SetStaticMesh (Variables|Default|GetMesh) (Variables|Default|GetNewMesh))
  (Rendering|Material|SetMaterial (Variables|Default|GetMesh) 0 "/Game/CustomMaps/UGC2768651799/PushAdvancedPack/ClassTools/Tools/Meshes/Materials/M_SplineArcMat.M_SplineArcMat"))

(fn OnRepHealthFull
  (if (Variables|Default|GetHealthFull)
    (CallFunction|SetWaitingMaterial)
    (CallFunction|SpawnArtillery)
    (else
      (CallFunction|SetCollisions))))