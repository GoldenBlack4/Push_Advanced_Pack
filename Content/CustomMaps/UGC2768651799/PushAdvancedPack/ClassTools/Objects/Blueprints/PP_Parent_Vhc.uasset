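; Parent Blueprint for a placed vehicle construction site that engineers build by hitting it with the CI_EngineerTool hammer.
; Server-side hammer overlaps add health once per swing and play a wood-hit sound until HealthFull is set.
; Its OnRep swaps the material, waits until no pawns overlap, then the server spawns VehicleClass with copied tags and destroys the site.
; Unfinished sites expire after LifeSpanUnconstructed, and a timer removes sites when the round ends.
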(event OnComponentBeginOverlap(Mesh)
  (params (OverlappedComponent :type Primitive%20Component%20Object%20Reference) (OtherActor :type Actor%20Object%20Reference) (OtherComp :type Primitive%20Component%20Object%20Reference) (OtherBodyIndex :type Integer) (bFromSweep :type Boolean) (SweepResult :type Hit%20Result%20Structure%20%28by%20ref%29))
  (Networking|SwitchHasAuthority
    (:Authority
      (bind _asci_engineer_tool (Utilities|Casting|CastToCI_EngineerTool OtherActor))
      (if (== (Variables|/Game/CustomMaps/UGC2768651799/PushAdvancedPack/ClassTools/Tools/Blueprints/CI_EngineerTool.CI_EngineerTool_C|GetHammerCollision _asci_engineer_tool) OtherComp)
        (if (not (Variables|Default|GetHealthFull))
          (Utilities|FlowControl|DoOnce false
            (:Completed
              (bind _output_get (Variables|Default|SetHealth (+ (Variables|Default|GetHealth) 25.0)))
              (CallFunction|RepairSound (Transformation|GetWorldLocation (Variables|/Game/CustomMaps/UGC2768651799/PushAdvancedPack/ClassTools/Tools/Blueprints/CI_EngineerTool.CI_EngineerTool_C|GetHammerCollision _asci_engineer_tool)))
              (Variables|Default|SetHealthFull (>= _output_get (Variables|Default|GetMaxHealth))))))))))

(event OnComponentEndOverlap(Mesh)
  (params (OverlappedComponent :type Primitive%20Component%20Object%20Reference) (OtherActor :type Actor%20Object%20Reference) (OtherComp :type Primitive%20Component%20Object%20Reference) (OtherBodyIndex :type Integer))
  (Networking|SwitchHasAuthority
    (:Authority
      (bind _asci_engineer_tool (Utilities|Casting|CastToCI_EngineerTool OtherActor))
      (Utilities|IsValid (Variables|/Game/CustomMaps/UGC2768651799/PushAdvancedPack/ClassTools/Tools/Blueprints/CI_EngineerTool.CI_EngineerTool_C|GetHammerCollision _asci_engineer_tool)
        (:Is%20Valid
          (Utilities|FlowControl|DoOnce false) ; enters at Reset
        )))))

(event Custom|SpawnVehicle
  (bind _returnvalue (Transformation|GetActorTransform))
  (Utilities|FlowControl|Delay 0.5)
  (bind _returnvalue_2 (Game|SpawnActorfromClass (Variables|Default|GetVehicleClass) (Math|Transform|MakeTransform (Math|Vector|MakeVector (.x (.location _returnvalue)) (.y (.location _returnvalue)) (+ (.z (.location _returnvalue)) 1e+02)) (.rotation _returnvalue) (.scale _returnvalue)) "AlwaysSpawn" 0 0))
  (Variables|/Script/Engine.Actor|SetTags _returnvalue_2 (Variables|Actor|GetTags))
  (Utilities|FlowControl|Delay 0.2)
  (Actor|DestroyActor))

(event Custom|RepairSound
  (params (Location :type Vector))
  ;[1 1 1] Sounds
  (Audio|PlaySoundatLocation "/Game/CustomMaps/UGC2768651799/PushAdvancedPack/ClassTools/Tools/Sounds/S_WoodHit.S_WoodHit" Location "0, 0, 0" 1.0 1.0 0.0 0 0 0))

(event Custom|PushEndRoundCheck
  (bind _returnvalue (Class|PavlovLibrary|GetGameLogic))
  (Utilities|IsValid _returnvalue
    (:Is%20Valid
      (switch Utilities|FlowControl|Switch|SwitchonEPavlovRoundState (Class|PavlovGameLogic|GetRoundState _returnvalue)
        (:Ended
          (Actor|DestroyActor))))))

(event Custom|SetMeshMaterial
  ;[1 1 1] Replicating
  (Rendering|Material|SetMaterial (Variables|Default|GetMesh) 0 (Variables|Default|GetWaitingMaterial))
  (if (> (Utilities|Array|Length (Collision|GetOverlappingActors (Variables|Default|GetMesh) "/Script/Engine.Pawn" :!class /Script/Engine.PrimitiveComponent)) 0) :!label _label
    (Utilities|FlowControl|Delay 1.0)
    (goto _label)
    (else
      (Networking|SwitchHasAuthority
        (:Authority
          (CallFunction|SpawnVehicle))))))

(event Custom|SetConstructMaterial
  (bind _mesh (Variables|Default|GetMesh))
  ;[1 1 1] Replicating
  (Collision|SetCollisionResponsetoAllChannels _mesh "ECR_Overlap")
  (Collision|SetCollisionResponsetoChannel _mesh "ECC_Visibility" "ECR_Block"))

(event EventBeginPlay
  (Networking|SwitchHasAuthority
    (:Authority
      (Utilities|Time|SetTimerbyEvent (delegate Custom|PushEndRoundCheck) 3.0 true)
      (Variables|Default|SetHealthFull false)
      (Utilities|FlowControl|Delay (Variables|Default|GetLifeSpanUnconstructed))
      (if (not (Variables|Default|GetHealthFull))
        (Actor|DestroyActor)))))

(fn ConstructionScript
  (Components|StaticMesh|SetStaticMesh (Variables|Default|GetMesh) (Variables|Default|GetNewMesh))
  (Rendering|Material|SetMaterial (Variables|Default|GetMesh) 0 "/Game/CustomMaps/UGC2768651799/PushAdvancedPack/ClassTools/Tools/Meshes/Materials/M_SplineArcMat.M_SplineArcMat"))

(fn OnRepHealthFull
  (if (Variables|Default|GetHealthFull)
    (CallFunction|SetMeshMaterial)
    (else
      (CallFunction|SetConstructMaterial))))