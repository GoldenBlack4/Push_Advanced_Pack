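; Parent Blueprint for engineer-built props that start as overlap-only construction ghosts and despawn if not completed in time or when the round ends.
; On the server, engineer hammer overlaps add health until built, or remove it in destroy mode.
; Replicated HealthFull switches material and collision, waiting for pawns to clear before blocking.
; Built props take damage only from name-matched explosives; barbed wire variants just play hit sounds, as pawn damage is unwired.
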(event OnComponentBeginOverlap(Mesh)
  (params (OverlappedComponent :type Primitive%20Component%20Object%20Reference) (OtherActor :type Actor%20Object%20Reference) (OtherComp :type Primitive%20Component%20Object%20Reference) (OtherBodyIndex :type Integer) (bFromSweep :type Boolean) (SweepResult :type Hit%20Result%20Structure%20%28by%20ref%29))
  ;[1 1 1] Construction
  (Networking|SwitchHasAuthority
    (:Authority
      (bind _asci_engineer_tool (Utilities|Casting|CastToCI_EngineerTool OtherActor))
      (if (== (Variables|/Game/CustomMaps/UGC2768651799/PushAdvancedPack/ClassTools/Tools/Blueprints/CI_EngineerTool.CI_EngineerTool_C|GetHammerCollision _asci_engineer_tool) OtherComp)
        (if (Variables|Default|GetHealthFull)
          (if (Variables|/Game/CustomMaps/UGC2768651799/PushAdvancedPack/ClassTools/Tools/Blueprints/CI_EngineerTool.CI_EngineerTool_C|GetDestroyMode _asci_engineer_tool)
            (bind _output_get (Variables|Default|SetHealth (- (Variables|Default|GetHealth) 1e+01)))
            (CallFunction|DestroySound (Transformation|GetWorldLocation (Variables|/Game/CustomMaps/UGC2768651799/PushAdvancedPack/ClassTools/Tools/Blueprints/CI_EngineerTool.CI_EngineerTool_C|GetHammerCollision _asci_engineer_tool)))
            (if (<= _output_get 0.0)
              (Actor|DestroyActor)))
          (else
            (Utilities|FlowControl|DoOnce false
              (:Completed
                (bind _output_get_2 (Variables|Default|SetHealth (+ (Variables|Default|GetHealth) 2e+01)))
                (CallFunction|RepairSound (Transformation|GetWorldLocation (Variables|/Game/CustomMaps/UGC2768651799/PushAdvancedPack/ClassTools/Tools/Blueprints/CI_EngineerTool.CI_EngineerTool_C|GetHammerCollision _asci_engineer_tool)))
                (Variables|Default|SetHealthFull (>= _output_get_2 (Variables|Default|GetMaxHealth)))))))))))

(event OnComponentEndOverlap(Mesh)
  (params (OverlappedComponent :type Primitive%20Component%20Object%20Reference) (OtherActor :type Actor%20Object%20Reference) (OtherComp :type Primitive%20Component%20Object%20Reference) (OtherBodyIndex :type Integer))
  ;[1 1 1] Construction
  (Networking|SwitchHasAuthority
    (:Authority
      (bind _asci_engineer_tool (Utilities|Casting|CastToCI_EngineerTool OtherActor))
      (Utilities|IsValid (Variables|/Game/CustomMaps/UGC2768651799/PushAdvancedPack/ClassTools/Tools/Blueprints/CI_EngineerTool.CI_EngineerTool_C|GetHammerCollision _asci_engineer_tool)
        (:Is%20Valid
          (Utilities|FlowControl|DoOnce false) ; enters at Reset
        )))))

(event OnComponentHit(Mesh)
  (params (HitComponent :type Primitive%20Component%20Object%20Reference) (OtherActor :type Actor%20Object%20Reference) (OtherComp :type Primitive%20Component%20Object%20Reference) (NormalImpulse :type Vector :default "0, 0, 0") (Hit :type Hit%20Result%20Structure%20%28by%20ref%29))
  (bind _self self)
  (bind _returnvalue (Utilities|GetClass _self))
  ;[1 1 1] Damage when hit (Barbed Wires only)
  (if (or (== _returnvalue "/Game/CustomMaps/UGC2768651799/PushAdvancedPack/ClassTools/Objects/Blueprints/PPC_Barbedwire1.PPC_Barbedwire1_C") (== _returnvalue "/Game/CustomMaps/UGC2768651799/PushAdvancedPack/ClassTools/Objects/Blueprints/PPC_Barbedwire2.PPC_Barbedwire2_C"))
    (Utilities|FlowControl|DoOnce false :!label _label
      (:Completed
        (CallFunction|PlayhitSound)
        (Utilities|FlowControl|Delay 1.0)
        (goto _label Reset)))))

(event Custom|DamagePawn
  (params (DamagedActor :type Actor%20Object%20Reference))
  ;[1 1 1] Damage when hit (Barbed Wires only)
  (bind _aspawn (Utilities|Casting|CastToPawn DamagedActor))
  (Game|Damage|ApplyDamage _aspawn 1e+01 (Game|GetInstigatorController) self))

(event Custom|PlayHitSound
  ;[1 1 1] Sounds
  (Audio|SpawnSoundatLocation "/Game/CustomMaps/UGC2768651799/PushAdvancedPack/ClassTools/Tools/Sounds/BarbedWire_Cue.BarbedWire_Cue" (Transformation|GetActorLocation) "0, 0, 0" 1.0 1.0 0.0 0 0))

(event Custom|DestroySound
  (params (Location :type Vector))
  ;[1 1 1] Sounds
  (Audio|PlaySoundatLocation "/Game/CustomMaps/UGC2768651799/PushAdvancedPack/ClassTools/Tools/Sounds/S_WoodHit.S_WoodHit" Location "0, 0, 0" 1.0 0.5 0.0 0 0 0))

(event Custom|RepairSound
  (params (Location :type Vector))
  ;[1 1 1] Sounds
  (Audio|PlaySoundatLocation "/Game/CustomMaps/UGC2768651799/PushAdvancedPack/ClassTools/Tools/Sounds/S_WoodHit.S_WoodHit" Location "0, 0, 0" 1.0 1.0 0.0 0 0 0))

(event Custom|PushEndRoundCheck
  (bind _returnvalue (Class|PavlovLibrary|GetGameLogic))
  ;[1 1 1] Begin play
  (Utilities|IsValid _returnvalue
    (:Is%20Valid
      (switch Utilities|FlowControl|Switch|SwitchonEPavlovRoundState (Class|PavlovGameLogic|GetRoundState _returnvalue)
        (:Ended
          (Actor|DestroyActor))))))

(event Custom|SetMeshMaterial
  (bind _mesh (Variables|Default|GetMesh))
  ;[1 1 1] Replicating
  (Rendering|Material|SetMaterial (Variables|Default|GetMesh) 0 (Variables|Default|GetWaitingMaterial))
  (if (> (Utilities|Array|Length (Collision|GetOverlappingActors (Variables|Default|GetMesh) "/Script/Engine.Pawn" :!class /Script/Engine.PrimitiveComponent)) 0) :!label _label
    (Utilities|FlowControl|Delay 1.0)
    (goto _label)
    (else
      (Rendering|Material|SetMaterial _mesh 0 (Variables|Default|GetDefaultMat))
      (Collision|SetCollisionResponsetoAllChannels _mesh "ECR_Block"))))

(event Custom|SetConstructMaterial
  (bind _mesh (Variables|Default|GetMesh))
  ;[1 1 1] Replicating
  (Collision|SetCollisionResponsetoAllChannels _mesh "ECR_Overlap")
  (Collision|SetCollisionResponsetoChannel _mesh "ECC_Visibility" "ECR_Block"))

(event EventBeginPlay
  ;[1 1 1] Begin play
  (Networking|SwitchHasAuthority
    (:Authority
      (Utilities|Time|SetTimerbyEvent (delegate Custom|PushEndRoundCheck) 3.0 true)
      (Variables|Default|SetHealthFull false)
      (Utilities|FlowControl|Delay (Variables|Default|GetLifeSpanUnconstructed))
      (if (not (Variables|Default|GetHealthFull))
        (Actor|DestroyActor)))))

(event Game|Damage|EventAnyDamage
  (params (Damage :type Float%20%28single-precision%29) (DamageType :type Damage%20Type%20Object%20Reference) (InstigatedBy :type Controller%20Object%20Reference) (DamageCauser :type Actor%20Object%20Reference))
  (bind _returnvalue (Utilities|GetDisplayName DamageCauser))
  ;[1 1 1] Damages
  (if (Variables|Default|GetHealthFull)
    (if (Math|Boolean|ORBoolean (Utilities|String|StartsWith _returnvalue "Rocket") (Utilities|String|StartsWith _returnvalue "Grenade_") (Utilities|String|StartsWith _returnvalue "Shell_") (Utilities|String|StartsWith _returnvalue "BP_ArtilleryProjectile") (Utilities|String|StartsWith _returnvalue "BP_Bomb"))
      (bind _output_get (Variables|Default|SetHealth (- (Variables|Default|GetHealth) Damage)))
      (if (<= _output_get 0.0)
        (Actor|DestroyActor)))))

(fn ConstructionScript
  (Components|StaticMesh|SetStaticMesh (Variables|Default|GetMesh) (Variables|Default|GetNewMesh))
  (Rendering|Material|SetMaterial (Variables|Default|GetMesh) 0 "/Game/CustomMaps/UGC2768651799/PushAdvancedPack/ClassTools/Tools/Meshes/Materials/M_SplineArcMat.M_SplineArcMat"))

(fn OnRepHealthFull
  (if (Variables|Default|GetHealthFull)
    (CallFunction|SetMeshMaterial)
    (else
      (CallFunction|SetConstructMaterial))))