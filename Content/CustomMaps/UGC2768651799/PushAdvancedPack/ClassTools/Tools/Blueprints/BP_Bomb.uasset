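; Homing bomb projectile that spins in flight and explodes on impact, with a ten-second lifespan.
; On BeginPlay it places a homing target at the given location, shifted to either side along local X when inaccurate.
; Server-side hits on anything but another bomb apply falloff radial damage sized by two sphere components, then destroy it.
; A multicast event handles explosion emitters, a decal and sound, plus a delayed distant boom.
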(event OnComponentHit(Collision)
  (params (HitComponent :type Primitive%20Component%20Object%20Reference) (OtherActor :type Actor%20Object%20Reference) (OtherComp :type Primitive%20Component%20Object%20Reference) (NormalImpulse :type Vector :default "0, 0, 0") (Hit :type Hit%20Result%20Structure%20%28by%20ref%29))
  (bind (_bblockinghit _binitialoverlap _time _distance _location _impactpoint _normal) (Collision|BreakHitResult Hit))
  (Networking|SwitchHasAuthority
    (:Authority
      (Utilities|FlowControl|DoOnce false
        (:Completed
          (if (not (== (Utilities|GetClass OtherActor) "BP_Bomb_C"))
            (Class|GameplayStatics|ApplyRadialDamagewithFalloff (Variables|Default|GetDamage) 0.0 _impactpoint (Components|Sphere|GetScaledSphereRadius (Variables|Default|GetInnerExplosionRadius)) (Components|Sphere|GetScaledSphereRadius (Variables|Default|GetOuterExplosionRadius)) 2.0 "/Game/CustomMaps/UGC2768651799/PushAdvancedPack/Artillery/Common/Blueprints/DamageType_Mine.DamageType_Mine_C" 0 self (Game|GetInstigatorController) "ECC_Visibility")
            (CallFunction|FXMulticast _impactpoint _normal)
            (Actor|DestroyActor)))))))

(event Custom|FX_Multicast
  (params (Location :type Vector) (Normal :type Vector))
  (Audio|Components|Audio|Stop (Variables|Default|GetBuzzingSound))
  (Development|SetHiddeninGame (Variables|Default|GetBombMesh) true true)
  (Collision|SetCollisionEnabled (Variables|Default|GetCollision) "NoCollision")
  (Effects|SpawnEmitteratLocation (Variables|Default|GetFireEmitter) Location "0, 0, 0" "10.000000,10.000000,10.000000")
  (Effects|SpawnEmitteratLocation (Variables|Default|GetFireEmitter2) Location "0, 0, 0" "10.000000,10.000000,10.000000")
  (Audio|PlaySoundatLocation (Variables|Default|GetBulletExplosion) Location "0, 0, 0" 1.0 (Math|Random|RandomFloatinRange 0.5 1.0) 0.0 0 0 0)
  (Rendering|Decal|SpawnDecalatLocation (Variables|Default|GetExplosionDecal) (Math|Conversions|ToVector(Float) (Components|Sphere|GetScaledSphereRadius (Variables|Default|GetOuterExplosionRadius))) Location (Math|Rotator|MakeRotfromX Normal) 1e+01)
  (Utilities|FlowControl|Delay 3.0)
  (Audio|PlaySoundatLocation (Variables|Default|GetBulletDistantExplosion) Location "0, 0, 0" 1.0 1.0 0.0 0 0 0))

(event EventTick
  (params (DeltaSeconds :type Float%20%28single-precision%29))
  (Transformation|AddLocalRotation (Variables|Default|GetBombMesh) "0.000000,0.000000,10.000000" false false))

(event EventBeginPlay
  (bind _target (Variables|Default|GetTarget))
  (Collision|IgnoreActorwhenMoving (Variables|Default|GetCollision) self true)
  (Actor|SetLifeSpan 1e+01)
  (if (Variables|Default|GetIsAccurate)
    (Transformation|SetWorldLocation (Variables|Default|GetTarget) (Variables|Default|GetTargetLocation) false true)
    (else
      (Transformation|SetWorldLocation _target (Variables|Default|GetTargetLocation) false true)
      (Transformation|AddRelativeLocation _target (Math|Vector|MakeVector (select (Variables|Default|GetIsFirst) -3e+03 3e+03) 0.0 0.0) false true)))
  (Variables|/Script/Engine.ProjectileMovementComponent|SetHomingTargetComponent (Variables|Default|GetProjectileMovement) (Variables|Default|GetTarget))
  (Transformation|SetWorldRotation (Variables|Default|GetBombMesh) (Math|Rotator|FindLookatRotation (Transformation|GetWorldLocation (Variables|Default|GetBombMesh)) (Transformation|GetWorldLocation (Variables|Default|GetTarget))) false true))

(fn ConstructionScript)