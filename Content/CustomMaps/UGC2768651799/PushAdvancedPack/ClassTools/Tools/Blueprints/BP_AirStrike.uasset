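; Air strike actor that flies a Stuka or Spitfire, chosen by team, over a target point to drop a bomb.
; On authority, BeginPlay sets a random heading, builds a team-specific spline (steep dive for Stuka), then launches after a delay.
; A timeline eases the plane along the spline, spins the propeller and fades engine audio.
; Near mid-flight, authority spawns one BP_Bomb at the bombdrop socket, aimed at the target.
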(event Custom|SpawnBombs
  (bind _plane (Variables|Default|GetPlane))
  (bind _returnvalue (Transformation|GetSocketTransform _plane "bombdrop" "RTS_World"))
  (Game|SpawnActorfromClass "/Game/CustomMaps/UGC2768651799/PushAdvancedPack/ClassTools/Tools/Blueprints/BP_Bomb.BP_Bomb_C" (Math|Transform|MakeTransform (.location _returnvalue) (.rotation _returnvalue) "1,1,1") "AlwaysSpawn" (Components|GetOwner) (Variables|Default|GetSplineMiddle) true false (Game|GetInstigator)))

(event Custom|StartPlane
  (params (NewTransformLocation :type Vector%20%28by%20ref%29) (TeamID :type Integer))
  (bind _output_get (Variables|Default|SetSplineMiddle NewTransformLocation))
  (bind _output_get_2 (Variables|Default|SetTeamID TeamID))
  (CallFunction|TransformReplicate _output_get _output_get_2 (Math|Rotator|MakeRotator 0.0 0.0 (Math|Random|RandomFloatinRange 0.0 3.6e+02)))
  (Utilities|FlowControl|Delay 5.0)
  (CallFunction|SpawnPlane))

(event Custom|SpawnPlane
  (bind _spline (Variables|Default|GetSpline))
  (bind _plane (Variables|Default|GetPlane))
  (bind _returnvalue (Transformation|GetWorldTransform _plane))
  ;[1 1 1] Plane Spline Line
  (Development|SetHiddeninGame (Variables|Default|GetPlane) false true)
  (Audio|Components|Audio|FadeIn (Variables|Default|GetAudio) 3.0 1.0 0.0 :!class /Script/Engine.AudioComponent)
  (bind _alpha (Timeline|Timeline_0 PlayFromStart)
    (:Update
      (Variables|Default|SetAlpha _alpha)
      (Transformation|SetWorldTransform (Variables|Default|GetPlane) (Math|Transform|MakeTransform (Math|Interpolation|VInterpTo (.location _returnvalue) (Spline|GetLocationatDistanceAlongSpline _spline (Math|Float|Lerp 0.0 (Spline|GetSplineLength (Variables|Default|GetSpline)) (Variables|Default|GetAlpha)) "World") (Variables|Default|GetAlpha) 1.0) (Math|Interpolation|RInterpTo (.rotation _returnvalue) (Spline|GetRotationatDistanceAlongSpline _spline (Math|Float|Lerp 0.0 (Spline|GetSplineLength (Variables|Default|GetSpline)) (Variables|Default|GetAlpha)) "World") (Variables|Default|GetAlpha) 1.0) "1,1,1") false false)
      (Transformation|AddLocalRotation (Variables|Default|GetPropeller) "0, 0,10.000000" false false)
      (Networking|SwitchHasAuthority
        (:Authority
          (if (Math|Float|NearlyEqual(Float) (Variables|Default|GetAlpha) 0.45 0.01)
            (Utilities|FlowControl|DoOnce false
              (:Completed
                (CallFunction|SpawnBombs)))))))
    (:Finished
      (Audio|Components|Audio|FadeOut (Variables|Default|GetAudio) 3.0 0.0 :!class /Script/Engine.AudioComponent)
      (Development|SetHiddeninGame (Variables|Default|GetPlane) true true)
      (Transformation|ResetRelativeTransform (Variables|Default|GetPlane)))))

(event Custom|TransformReplicate
  (params (SplineMiddle :type Vector) (Team :type Integer) (ActorRotation :type Rotator))
  (CallFunction|SplineSpitfire SplineMiddle Team)
  (Transformation|SetActorRotation ActorRotation)
  (Components|StaticMesh|SetStaticMesh (Variables|Default|GetPlane) (Utilities|Select :Index Team :Option%200 "/Game/CustomMaps/UGC2768651799/PushAdvancedPack/ClassTools/Tools/Meshes/GER_Stuka/SM_Plane_Ju87Stuka_01.SM_Plane_Ju87Stuka_01" :Option%201 "/Game/CustomMaps/UGC2768651799/PushAdvancedPack/ClassTools/Tools/Meshes/US_Spitfire/spitfire.spitfire"))
  (Audio|Components|Audio|SetSound (Variables|Default|GetAudio) (Utilities|Select :Index Team :Option%200 "/Game/CustomMaps/UGC2768651799/PushAdvancedPack/ClassTools/Tools/Sounds/Stuka_Cue.Stuka_Cue" :Option%201 "/Game/CustomMaps/UGC2768651799/PushAdvancedPack/ClassTools/Tools/Sounds/SpitFire_Cue.Spitfire_Cue")))

(event EventBeginPlay
  ;[1 0 0] Debug
  (Networking|SwitchHasAuthority
    (:Authority
      (Utilities|FlowControl|Delay 1.0)
      (Utilities|IsValid (Class|PavlovLibrary|GetGameLogic)
        (:Is%20Valid
          (CallFunction|StartPlane (Variables|Default|GetSplineMiddle) (Variables|Default|GetTeamID)))
        (:Is%20Not%20Valid
          (bind _output_get (Variables|Default|SetSplineMiddle (Transformation|GetActorLocation)))
          (CallFunction|StartPlane _output_get (Variables|Default|GetTeamID)))))))

(fn ConstructionScript
  (Transformation|AttachComponentToComponent (Variables|Default|GetPropeller) (Variables|Default|GetPlane) "propeller" "SnapToTarget" "SnapToTarget" "KeepWorld" true))

(fn SplineSpitfire
  (params (SplineMiddle :type Vector) (Team :type Integer))
  (bind (_x _y _z) (Math|Vector|BreakVector SplineMiddle))
  (bind (_x_2 _y_2 _z_2) (Math|Vector|BreakVector SplineMiddle))
  (bind _spline (Variables|Default|GetSpline))
  (bind _spline_2 (Variables|Default|GetSpline))
  (if (== Team 1)
    (bind _output_get (Variables|Default|SetSpitFireSplineStart (+ SplineMiddle "-80000.000000, 0,20000.000000")))
    (Transformation|SetWorldTransform (Variables|Default|GetSpline) (Math|Transform|MakeTransform _output_get "0, 0, 0" "1,1,1") false false)
    (Spline|AddSplinePoint _spline_2 (Math|Vector|MakeVector _x _y (+ _z 6e+03)) "World" true)
    (bind _output_get_2 (Variables|Default|SetSpitFireSplineEnd (+ SplineMiddle "80000.000000, 0,20000.000000")))
    (Spline|AddSplinePoint _spline_2 _output_get_2 "World" true)
    (else
      (bind _output_get_3 (Variables|Default|SetStukaFireSplineStart (+ SplineMiddle "-20000.000000, 0,80000.000000")))
      (Transformation|SetWorldTransform (Variables|Default|GetSpline) (Math|Transform|MakeTransform _output_get_3 "0, 0, 0" "1,1,1") false false)
      (Spline|AddSplinePoint _spline (Math|Vector|MakeVector _x_2 _y_2 (+ _z_2 1e+04)) "World" true)
      (bind _output_get_4 (Variables|Default|SetStukaSplineEnd (+ SplineMiddle "80000.000000, 0,20000.000000")))
      (Spline|AddSplinePoint _spline _output_get_4 "World" true))))