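; Commander's handheld monocular for a Pavlov mod that calls airstrikes or places team markers at the aimed point.
; The client line-traces each tick and sends the point to the server, which spawns an airstrike if the team's aircraft is available or replaces that team's same-type marker from DT_Markers.
; Pickup binds owner and team, flips the layout by hand and creates a scene capture.
; Other pawns are forced to drop it, and dropped tools self-destroy after a delay.
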(event Custom|Deactivate
  (bind _scenecapture (Variables|Default|GetSceneCapture))
  ;[1 1 1] ActivateDeactivate SceneCapture
  (Utilities|IsValid _scenecapture
    (:Is%20Valid
      (Components|DestroyComponent _scenecapture))))

(event Custom|Activate
  ;[1 1 1] ActivateDeactivate SceneCapture
  (CallFunction|CreateRenderTarget))

(event Custom|ObjectSelection_Server
  (params (InputPin :type Float%20%28single-precision%29))
  ;[1 1 1] Object Selection
  (switch int (Variables|Default|GetMode)
    (:1
      (if (> InputPin 0.1)
        (Utilities|FlowControl|DoOnce false :!label _label
          (:Completed
            (CallFunction|NextMarker)
            (CallFunction|NextMeshSound)
            (Utilities|FlowControl|Delay 0.2)
            (goto _label Reset)))
        (elif (not (> InputPin -0.1))
          (Utilities|FlowControl|DoOnce false :!label _label_2
            (:Completed
              (CallFunction|PreviousMarker)
              (CallFunction|PreviousMeshSound)
              (Utilities|FlowControl|Delay 0.2)
              (goto _label_2 Reset))))))))

(event Custom|EnableInputClient
  ;[0.4638 0.7848 1] Inputs
  ;;[1 1 1] Pick Up
  (Input|EnableInput (Game|GetPlayerController 0)))

(event Custom|NextMarker
  ;[0 0 0] Markers Selection Logic
  (bind _output_get (Variables|Default|SetMarker_Selected (Utilities|Enum|ByteToEnumEnum_Markers (+ (Variables|Default|GetMarker_Selected) 1))))
  (if (== _output_get (Math|Conversions|ToByte(Integer) (|GetNumEnumEntries)))
    (bind _output_get_2 (Variables|Default|SetMarker_Selected (Utilities|Enum|ByteToEnumEnum_Markers (- (Variables|Default|GetMarker_Selected) (Math|Conversions|ToByte(Integer) (|GetNumEnumEntries)))))))
  (CallFunction|UpdateTextClient (Variables|Default|GetMode) _output_get_2))

(event Custom|PreviousMarker
  ;[0 0 0] Markers Selection Logic
  (bind _output_get (Variables|Default|SetMarker_Selected (Utilities|Enum|ByteToEnumEnum_Markers (- (Variables|Default|GetMarker_Selected) 1))))
  (if (== _output_get (Math|Conversions|ToByte(Integer) (|GetNumEnumEntries)))
    (bind _output_get_2 (Variables|Default|SetMarker_Selected (Utilities|Enum|ByteToEnumEnum_Markers (- (Math|Conversions|ToByte(Integer) (|GetNumEnumEntries)) 1)))))
  (CallFunction|UpdateTextClient (Variables|Default|GetMode) _output_get_2))

(event Custom|PreviousMeshSound
  ;[1 1 1] Sounds FX
  (Audio|PlaySound2D "/Game/CustomMaps/UGC2768651799/PushAdvancedPack/ClassTools/Tools/Sounds/S_SwitchMesh.S_SwitchMesh" 1.0 0.5 0.0 0 0))

(event Custom|NextMeshSound
  ;[1 1 1] Sounds FX
  (Audio|PlaySound2D "/Game/CustomMaps/UGC2768651799/PushAdvancedPack/ClassTools/Tools/Sounds/S_SwitchMesh.S_SwitchMesh" 1.0 1.0 0.0 0 0))

(event Custom|OnDropServer
  ;[0.4638 0.7848 1] Inputs
  ;;[1 1 1] Drop
  (CallFunction|DisableInputClient)
  (CallFunction|DisableTick)
  (CallFunction|DestroyServer))

(event Custom|Flip
  (params (Dominant :type Boolean) (RightHanded :type Boolean))
  ;[1 1 1] FlipUnflip Monocular
  (if Dominant ; Dominant?
    (if RightHanded ; RightHanded?
      (CallFunction|UnflipMonocular :!label _label)
      (else
        (CallFunction|FlipMonocular :!label _label_2)))
    (elif RightHanded ; LeftHanded?
      (goto _label_2)
      (else
        (goto _label)))))

(event Custom|SwitchModeSound
  ;[1 1 1] Sounds FX
  (Audio|PlaySound2D "/Game/CustomMaps/UGC2768651799/PushAdvancedPack/ClassTools/Tools/Sounds/S_ModeSwitch.S_ModeSwitch" 1.0 1.0 0.0 0 0))

(event Custom|DisableTick
  ;[0.4638 0.7848 1] Inputs
  ;;[1 1 1] Drop
  (Actor|Tick|SetActorTickEnabled false)
  (Development|SetHiddeninGame (Variables|Default|GetText) true false))

(event Custom|DestroyServer
  ;[0.4638 0.7848 1] Inputs
  ;;[1 1 1] Drop
  (if (not (Variables|Default|GetDebugMode))
    (bind _returnvalue (Class|PavlovCustomItem|GetItemState))
    (if (Utilities|Enum|Equal(Enum) _returnvalue "InWorld")
      (Utilities|FlowControl|Delay (Variables|Default|GetDestroyOnDropDelay))
      (bind _returnvalue_2 (Class|PavlovCustomItem|GetItemState))
      (if (Utilities|Enum|Equal(Enum) _returnvalue_2 "InWorld")
        (CallFunction|DestroyMulticast)))))

(event Custom|SetImpactPoint_Server
  (params (Object%20Transform%20Location :type Vector) (Object%20Transform%20Rotation :type Rotator))
  ;[1 1 1] Tick
  (Variables|Default|SetObjectTransform (Math|Transform|MakeTransform Object%20Transform%20Location Object%20Transform%20Rotation "1,1,1")))

(event Custom|UnflipMonocular
  (bind _tool (Variables|Default|GetTool))
  ;[1 1 1] FlipUnflip Monocular
  (Components|StaticMesh|SetStaticMesh _tool "/Game/CustomMaps/UGC2768651799/PushAdvancedPack/ClassTools/Tools/Meshes/Monocular/Props/SM_Monocular02.SM_Monocular02")
  (Transformation|SetRelativeTransform _tool (Variables|Default|GetMono_UnflipTransform) false false)
  (Transformation|SetRelativeTransform (Variables|Default|GetSceneCaptureLocation) (Variables|Default|GetScene_UnflipTransform) false false)
  (Transformation|SetRelativeTransform (Variables|Default|GetText) (Variables|Default|GetText_UnflipTransform) false false))

(event Custom|OnPickUp_Server
  (params (OwnerPawn :type Pawn%20Object%20Reference) (PickedByDominant :type Boolean))
  ;[0.4638 0.7848 1] Inputs
  ;;[1 1 1] Pick Up
  (bind _output_get (Variables|Default|SetPickedByDominant PickedByDominant))
  (Utilities|Attribution OwnerPawn _output_get
    (:Good
      (CallFunction|EnableInputClient)
      (CallFunction|EnableTick)
      (CallFunction|Activate)
      (CallFunction|UpdateTextClient (Variables|Default|GetMode) (Variables|Default|GetMarker_Selected)))
    (:False
      (CallFunction|DestroyMulticast))))

(event Custom|DisableInputClient
  ;[0.4638 0.7848 1] Inputs
  ;;[1 1 1] Drop
  (CallFunction|Deactivate)
  (if (not (Variables|Default|GetDebugMode))
    (Input|DisableInput (Game|GetPlayerController 0))))

(event Custom|IsValidPointServer
  (params (IsValidDestination :type Boolean))
  ;[1 1 1] Tick
  (Variables|Default|SetIsValidPoint IsValidDestination))

(event Custom|OnUse_Server
  (bind _ownerpawn (Variables|Default|GetOwnerPawn))
  (bind _ownerpawn_2 (Variables|Default|GetOwnerPawn))
  (bind _objecttransform (Variables|Default|GetObjectTransform))
  (bind _ownerpawn_3 (Variables|Default|GetOwnerPawn))
  (bind _marker_selected (Variables|Default|GetMarker_Selected))
  (bind _returnvalue (Utilities|String|EnumtoString _marker_selected))
  (bind _returnvalue_2 (Utilities|String|StringToName _returnvalue))
  ;[0 0 0] Right Trigger Action
  (switch int (Variables|Default|GetMode)
    (:0
      ;;[0.1232 0.3635 1] AirStrike
      (if (Variables|Default|GetIsValidPoint)
        (Utilities|AircraftTeamAvailability
          (:SpawnPlane
            (Game|SpawnActorfromClass "/Game/CustomMaps/UGC2768651799/PushAdvancedPack/ClassTools/Tools/Blueprints/BP_AirStrike.BP_AirStrike_C" (Math|Transform|MakeTransform (.location _objecttransform) "0, 0, 0" "1,1,1") "AlwaysSpawn" 0 (Variables|Default|GetTeamID) (.location _objecttransform) _ownerpawn_2 :!label _label)
            (CallFunction|PlaySound (Variables|Default|GetTeamID) _ownerpawn_2)
            (Game|SpawnActorfromClass "/Game/CustomMaps/UGC2768651799/PushAdvancedPack/ClassTools/Tools/Markers/BP_Marker.BP_Marker_C" (Math|Transform|MakeTransform (.location _objecttransform) "0, 0, 0" "1,1,1") "AlwaysSpawn" _ownerpawn "/Game/CustomMaps/UGC2768651799/PushAdvancedPack/ClassTools/Tools/Markers/Materials/Marker_Airstrike_Mat.Marker_Airstrike_Mat" 15.0 "/Game/CustomMaps/UGC2768651799/PushAdvancedPack/ClassTools/Tools/Sounds/VR_click2.VR_click2" (Variables|Default|GetTeamID) (Variables|Default|GetTeamIDSwitched) _ownerpawn))
          (:CastFailed
            (goto _label))
          (:NotAvailable
            (CallFunction|UnavailableSound :!label _label_2)))
        (else
          (goto _label_2))))
    (:1
      ;;[0.3585 0.3841 1] Ping
      (if (and (Variables|Default|GetIsValidPoint) (Variables|Default|GetCanSetMarker))
        (bind _returnvalue_3 (Utilities|GetDataTableRow "/Game/CustomMaps/UGC2768651799/PushAdvancedPack/ClassTools/Tools/Markers/DT_Markers.DT_Markers" _returnvalue_2)
          (:then
            (bind _outactors (Actor|GetAllActorsOfClass "/Game/CustomMaps/UGC2768651799/PushAdvancedPack/ClassTools/Tools/Markers/BP_Marker.BP_Marker_C"))
            (for _array_element _outactors
              (if (and (Actor|ActorHasTag _array_element _returnvalue_2) (Actor|ActorHasTag _array_element (Utilities|String|StringToName (Utilities|String|ToString(Integer) (Variables|Default|GetTeamID)))))
                (Actor|DestroyActor _array_element)))
            (bind _returnvalue_4 (Game|SpawnActorfromClass "/Game/CustomMaps/UGC2768651799/PushAdvancedPack/ClassTools/Tools/Markers/BP_Marker.BP_Marker_C" (Math|Transform|MakeTransform (.location (Variables|Default|GetObjectTransform)) "0, 0, 0" "1,1,1") "AlwaysSpawn" _ownerpawn_3 (.material _returnvalue_3) (.lifespan _returnvalue_3) (.sound _returnvalue_3) (Variables|Default|GetTeamID) (Variables|Default|GetTeamIDSwitched) _ownerpawn_3))
            (Variables|/Script/Engine.Actor|SetTags _returnvalue_4 (Utilities|Array|MakeArray _returnvalue_2 (Utilities|String|StringToName (Utilities|String|ToString(Integer) (Variables|Default|GetTeamID)))))
            (Variables|Default|SetCanSetMarker false)
            (Utilities|FlowControl|Delay 3.0)
            (Variables|Default|SetCanSetMarker true)))))))

(event Custom|ChangeModeServer
  ;[0.4638 0.7848 1] Inputs
  ;;[1 1 1] Change Mode
  (CallFunction|SwitchModeSound)
  (Utilities|FlowControl|MultiGate false true 1
    (:Out%200
      (Variables|Default|SetMode 0))
    (:Out%201
      (Variables|Default|SetMode 1)))
  (CallFunction|UpdateTextClient (Variables|Default|GetMode) (Variables|Default|GetMarker_Selected)))

(event Custom|FlipMonocular
  (bind _tool (Variables|Default|GetTool))
  ;[1 1 1] FlipUnflip Monocular
  (Components|StaticMesh|SetStaticMesh _tool "/Game/CustomMaps/UGC2768651799/PushAdvancedPack/ClassTools/Tools/Meshes/Monocular/Props/SM_MonocularFlipped02.SM_MonocularFlipped02")
  (Transformation|SetRelativeTransform _tool (Variables|Default|GetMono_FlipTransform) false false)
  (Transformation|SetRelativeTransform (Variables|Default|GetSceneCaptureLocation) (Variables|Default|GetScene_FlipTransform) false false)
  (Transformation|SetRelativeTransform (Variables|Default|GetText) (Variables|Default|GetText_FlipTransform) false false))

(event Custom|UpdateTextClient
  (params (Mode :type Integer) (MarkerSelected :type Enum_Markers%20Enum :default "NewEnumerator19"))
  (bind _text (Variables|Default|GetText))
  ;[0 0 0] Switch Mode Logic
  (bind _output_get (Variables|Default|SetMode Mode))
  (switch int _output_get
    (:0
      (Rendering|Components|TextRender|SetText _text (Utilities|Text|ToText(String) "Call 
Airstrike")))
    (:1
      (Rendering|Components|TextRender|SetText _text (Utilities|Text|ToText(String) (Utilities|String|Append "Place marker" " 
" (Utilities|String|EnumtoString MarkerSelected))))
      (Rendering|Components|TextRender|SetTextRenderColor (Variables|Default|GetText) (Variables|Default|GetAirstrikeAvalaible)))))

(event Custom|Debug_ChangeTeam
  ;[1 0 0] debug
  (Utilities|FlowControl|FlipFlop
    (:A
      (Variables|Default|SetTeamID 1))
    (:B
      (Variables|Default|SetTeamID 0)))
  (Development|PrintString (Utilities|String|ToString(Integer) (Variables|Default|GetTeamID))))

(event Custom|DestroyMulticast
  ;[0.4638 0.7848 1] Inputs
  ;;[1 1 1] Drop
  (Actor|DestroyActor))

(event Custom|EnableTick
  ;[0.4638 0.7848 1] Inputs
  ;;[1 1 1] Pick Up
  (Actor|Tick|SetActorTickEnabled true)
  (Development|SetHiddeninGame (Variables|Default|GetText) false false))

(event Custom|PlaySound
  (params (TeamID :type Integer) (Pawn :type Pawn%20Object%20Reference))
  ;[1 1 1] Sounds FX
  (Audio|PlaySound2D (Utilities|Select :Index TeamID :Option%200 "/Game/CustomMaps/UGC2768651799/PushAdvancedPack/ClassTools/Tools/Sounds/Luftangriff.Luftangriff" :Option%201 "/Game/CustomMaps/UGC2768651799/PushAdvancedPack/ClassTools/Tools/Sounds/Radio_AirStrike1.Radio_AirStrike1") 0.5 1.0 0.0 0 Pawn))

(event Custom|UnavailableSound
  ;[1 1 1] Sounds FX
  (Audio|PlaySound2D "/Game/CustomMaps/UGC2768651799/PushAdvancedPack/Artillery/Common/Sound/VR_negative.VR_negative" 1.0 1.0 0.0 0 0))

(event EventBeginPlay
  ;[1 1 1] Begin Play
  (Networking|SwitchHasAuthority
    (:Authority
      (Utilities|FlowControl|Delay 1.0)
      (Utilities|IsValid (Class|PavlovLibrary|GetGameLogic)
        (:Is%20Valid
          (bind (_pawn _returnvalue) (Class|PavlovCustomItem|GetOwningPawn))
          (if _returnvalue
            (Variables|Default|SetOwnerPawn _pawn)
            (bind _returnvalue_2 (Class|PavlovCustomItem|GetItemState))
            (if (Utilities|Enum|Equal(Enum) _returnvalue_2 "InHand")
              (CallFunction|Activate)
              (else
                (CallFunction|Deactivate :!label _label)))
            (else
              (goto _label))))
        (:Is%20Not%20Valid
          ;[1 0 0] debug
          (Variables|Default|SetDebugMode true)
          (bind _output_get (Variables|Default|SetOwnerPawn (Game|Player|GetPlayerPawn 0)))
          (Actor|SetOwner _output_get)
          (Utilities|FlowControl|Delay 1.0)
          (CallFunction|UpdateTextClient (Variables|Default|GetMode) (Variables|Default|GetMarker_Selected))
          (CallFunction|EnableInputClient)
          (CallFunction|EnableTick)
          (CallFunction|Activate)
          (CallFunction|Flip true true))))))

(event EventOnDrop
  ;[0.4638 0.7848 1] Inputs
  ;;[1 1 1] Drop
  (CallFunction|OnDropServer))

(event EventOnUse
  ;[0.4638 0.7848 1] Inputs
  ;;[1 1 1] On Use
  (Utilities|FlowControl|DoOnce false :!label _label
    (:Completed
      (CallFunction|OnUseServer)
      (Utilities|FlowControl|Delay 0.5)
      (goto _label Reset))))

(event EventTick
  (params (DeltaSeconds :type Float%20%28single-precision%29))
  ;[1 1 1] Tick
  (Networking|SwitchHasAuthority
    (:Remote
      (bind (_impactpoint _returnvalue) (CallFunction|GroundTrace))
      (CallFunction|IsValidPointServer _returnvalue)
      (if _returnvalue
        (CallFunction|SetImpactPointServer _impactpoint "0, 0, 0")))))

(event EventOnPickup
  (params (Pawn :type Pawn%20Object%20Reference) (bDominant :type Boolean))
  ;[0.4638 0.7848 1] Inputs
  ;;[1 1 1] Pick Up
  (CallFunction|OnPickUpServer Pawn bDominant))

(event Input|ActionEvents|InputActionCycleFireModeRight
  (params (Key :type Key%20Structure))
  ;[0.4638 0.7848 1] Inputs
  ;;[1 1 1] Change Mode
  (:Pressed
    (Utilities|FlowControl|DoOnce false :!label _label
      (:Completed
        (CallFunction|ChangeModeServer)
        (Utilities|FlowControl|Delay 0.5)
        (goto _label Reset)))))

(event Input|ActionEvents|InputActionCycleFireModeLeft
  (params (Key :type Key%20Structure))
  ;[0.4638 0.7848 1] Inputs
  ;;[1 1 1] Change Mode
  (:Pressed
    (Utilities|FlowControl|DoOnce false :!label _label
      (:Completed
        (CallFunction|ChangeModeServer)
        (Utilities|FlowControl|Delay 0.5)
        (goto _label Reset)))))

(event Input|AxisEvents|InputAxisSpectatorMove_Y
  (params (AxisValue :type Float%20%28single-precision%29))
  ;[1 1 1] Object Selection
  (if (> (Math|Float|Absolute(Float) AxisValue) 0.7)
    (CallFunction|ObjectSelectionServer (* AxisValue -1.0))))

(event Input|MouseEvents|MiddleMouseButton
  (params (Key :type Key%20Structure))
  ;[1 0 0] debug
  (:Pressed
    (if (Variables|Default|GetDebugMode)
      ;[0.4638 0.7848 1] Inputs
      ;;[1 1 1] Change Mode
      (Utilities|FlowControl|DoOnce false :!label _label
        (:Completed
          (CallFunction|ChangeModeServer)
          (Utilities|FlowControl|Delay 0.5)
          (goto _label Reset))))))

(event Input|KeyboardEvents|Up
  (params (Key :type Key%20Structure))
  ;[1 0 0] debug
  (:Pressed
    (if (Variables|Default|GetDebugMode)
      (CallFunction|ObjectSelectionServer 1.2))))

(event Input|KeyboardEvents|Down
  (params (Key :type Key%20Structure))
  ;[1 0 0] debug
  (:Pressed
    (if (Variables|Default|GetDebugMode)
      (CallFunction|ObjectSelectionServer -1.2))))

(event Input|MouseEvents|LeftMouseButton
  (params (Key :type Key%20Structure))
  ;[1 0 0] debug
  (:Pressed
    (if (Variables|Default|GetDebugMode)
      ;[0.4638 0.7848 1] Inputs
      ;;[1 1 1] On Use
      (Utilities|FlowControl|DoOnce false :!label _label
        (:Completed
          (CallFunction|OnUseServer)
          (Utilities|FlowControl|Delay 0.5)
          (goto _label Reset))))))

(fn ConstructionScript
  (Components|StaticMesh|SetStaticMesh (Variables|Default|GetTool) "/Game/CustomMaps/UGC2768651799/PushAdvancedPack/ClassTools/Tools/Meshes/Monocular/Props/SM_Monocular02.SM_Monocular02")
  (Transformation|SetRelativeTransform (Variables|Default|GetTool) (Variables|Default|GetMono_UnflipTransform) false false)
  (Transformation|SetRelativeTransform (Variables|Default|GetSceneCaptureLocation) (Variables|Default|GetScene_UnflipTransform) false false)
  (Transformation|SetRelativeTransform (Variables|Default|GetText) (Variables|Default|GetText_UnflipTransform) false false))

(fn GroundTrace
  (bind _arrow (Variables|Default|GetArrow))
  (bind _returnvalue (Transformation|GetWorldLocation _arrow))
  (bind (_outhit _returnvalue_2) (Collision|LineTraceByChannel _returnvalue (+ _returnvalue (* (Math|Vector|GetForwardVector (Transformation|GetWorldRotation _arrow)) 1e+05)) "TraceTypeQuery1" false 0 "ForOneFrame"))
  (return (.ImpactPoint (Collision|BreakHitResult _outhit)) _returnvalue_2))

(fn CreateRenderTarget
  (Utilities|IsValid (Variables|Default|GetSceneCapture)
    (:Is%20Valid
      (Components|DestroyComponent (Variables|Default|GetSceneCapture)))
    (:Is%20Not%20Valid
      _))
  (bind _returnvalue (AddComponent|AddSceneCaptureComponent2D false (Transformation|GetRelativeTransform (Variables|Default|GetSceneCaptureLocation))))
  (Variables|Default|SetSceneCapture _returnvalue)
  (return))

(fn SwitchonTDM
  (params (Condition :type Boolean))
  (if (not Condition)
    (Variables|Default|SetTeamIDSwitched true)
    (if (== (Variables|Default|GetTeamID) 0)
      (Variables|Default|SetTeamID 1)
      (else
        (Variables|Default|SetTeamID 0)))))